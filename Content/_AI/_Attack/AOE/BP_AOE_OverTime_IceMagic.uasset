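; BP_AOE_OverTime_IceMagic is an ice magic area-of-effect attack, a child Blueprint meant to deal damage over time.
; The Trigger event, commented as continuous damage, only forwards to the parent, so the attack logic is inherited.
; BeginPlay sets the Color parameter on the Niagara component without calling the parent's BeginPlay.
; Overlap and Tick are disabled stubs, and the construction script only calls the parent.
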(event EventBeginPlay
  (Effects|Components|ParticleSystem|SetColorParameter (Variables|Default|GetNiagara) "Color" (Variables|Default|GetParam)))

(event Collision|EventActorBeginOverlap
  (params (OtherActor :type Actor%20Object%20Reference))
  (|CallParentFunction OtherActor) ; This node is disabled and will not be called.\nDrag off pins to build functionality.
)

(event EventTick
  (params (DeltaSeconds :type Float%20%28single-precision%29))
  (|CallParentFunction DeltaSeconds) ; This node is disabled and will not be called.\nDrag off pins to build functionality.
)

(event EventTrigger
  (|CallParentFunction))

(fn ConstructionScript
  (|CallParentFunction))