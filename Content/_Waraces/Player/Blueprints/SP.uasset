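; Player-side actor (SP) that manages red and blue team card slots and the display characters standing on them.
; It spawns BP_CardSlot actors per team, then spawns or removes BP_NPC_Display characters by team and index, storing each on its slot.
; Clearing all slots destroys the displays and red slots, but the blue loop calls DestroyActor on itself.
; Key 1 debug-prints each VRPawn_Main's hand-container interface name.
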(event Custom|生成角色槽位
  (Utilities|FlowControl|Sequence
    (:then_0
      (bind _槽位生成位置_ (CallFunction|取得角色槽位的生成位置 "NewEnumerator1"))
      (for (_array_element _array_index) _槽位生成位置_
        (bind _returnvalue (Game|SpawnActorfromClass "/Game/_Waraces/Cards/Card_UIs/CardSlot/BP_CardSlot.BP_CardSlot_C" _array_element "Undefined" 0 _array_index "NewEnumerator1" self false 0))
        (Utilities|Array|Add (Variables|Default|Get紅隊卡牌槽位) _returnvalue)))
    (:then_1
      (bind _槽位生成位置__2 (CallFunction|取得角色槽位的生成位置 "NewEnumerator2"))
      (for (_array_element_2 _array_index_2) _槽位生成位置__2
        (bind _returnvalue_2 (Game|SpawnActorfromClass "/Game/_Waraces/Cards/Card_UIs/CardSlot/BP_CardSlot.BP_CardSlot_C" _array_element_2 "Undefined" 0 _array_index_2 "NewEnumerator2" self false 0))
        (Utilities|Array|Add (Variables|Default|Get藍隊卡牌槽位) _returnvalue_2)))))

(event Custom|移除所有槽位
  (for _array_element (Variables|Default|Get紅隊卡牌槽位)
    (Actor|DestroyActor (Variables|/Game/_Waraces/Cards/Card_UIs/CardSlot/BP_CardSlot.BP_CardSlot_C|Get目前生成在槽位上的展示角色 _array_element))
    (Actor|DestroyActor _array_element))
  (for _array_element_2 (Variables|Default|Get藍隊卡牌槽位)
    (Actor|DestroyActor (Variables|/Game/_Waraces/Cards/Card_UIs/CardSlot/BP_CardSlot.BP_CardSlot_C|Get目前生成在槽位上的展示角色 _array_element_2))
    (Actor|DestroyActor)))

(event Custom|生成槽位上的角色
  (params (序號 :type Integer) (角色 :type E_NPC%20Enum :default "NewEnumerator0") (陣營 :type E_Team%20Enum :default "NewEnumerator0"))
  (bind _紅隊卡牌槽位 (Variables|Default|Get紅隊卡牌槽位))
  (bind _藍隊卡牌槽位 (Variables|Default|Get藍隊卡牌槽位))
  (bind _returnvalue (Utilities|Select :Index 陣營 :NewEnumerator0 0 :NewEnumerator1 _紅隊卡牌槽位 :NewEnumerator2 _藍隊卡牌槽位))
  (bind _output (Utilities|Array|Get(acopy) _returnvalue 序號))
  (bind _returnvalue_2 (Game|SpawnActorfromClass "/Game/_AI/NPC_Base/BP_NPC_Display.BP_NPC_Display_C" (|取得展示角色生成位置 _output 1e+02) "Undefined" 0 角色 陣營 (CallFunction|取得指定陣營的玩家 陣營) 序號 _output false 0))
  (Variables|/Game/_Waraces/Cards/Card_UIs/CardSlot/BP_CardSlot.BP_CardSlot_C|Set目前生成在槽位上的展示角色 _output _returnvalue_2))

(event Custom|移除指定陣營卡牌槽位上的角色
  (params (序號 :type Integer) (陣營 :type E_Team%20Enum :default "NewEnumerator0"))
  (bind _紅隊卡牌槽位 (Variables|Default|Get紅隊卡牌槽位))
  (bind _藍隊卡牌槽位 (Variables|Default|Get藍隊卡牌槽位))
  (bind _returnvalue (Utilities|Select :Index 陣營 :NewEnumerator0 0 :NewEnumerator1 _紅隊卡牌槽位 :NewEnumerator2 _藍隊卡牌槽位))
  (bind _output (Utilities|Array|Get(acopy) _returnvalue 序號))
  (bind _目前生成在槽位上的展示角色 (Variables|/Game/_Waraces/Cards/Card_UIs/CardSlot/BP_CardSlot.BP_CardSlot_C|Get目前生成在槽位上的展示角色 _output)
    (:then
      (Actor|DestroyActor _目前生成在槽位上的展示角色)
      (Variables|/Game/_Waraces/Cards/Card_UIs/CardSlot/BP_CardSlot.BP_CardSlot_C|Set目前生成在槽位上的展示角色 _output 0))
    (:else)))

(event EventBeginPlay)

(event Collision|EventActorBeginOverlap
  (params (OtherActor :type Actor%20Object%20Reference)))

(event EventTick
  (params (DeltaSeconds :type Float%20%28single-precision%29)))

(event Input|KeyboardEvents|1
  (params (Key :type Key%20Structure))
  (:Pressed
    (bind _outactors (Actor|GetAllActorsOfClass "/Game/_Waraces/Player/Blueprints/VRPawn_Main.VRPawn_Main_C"))
    (for _array_element _outactors
      (Development|PrintString (Utilities|GetDisplayName (Variables|/Game/_Waraces/Player/Blueprints/VR_Pawn_Base.VR_Pawn_Base_C|Get玩家手牌容器介面 _array_element))))))

(fn ConstructionScript)