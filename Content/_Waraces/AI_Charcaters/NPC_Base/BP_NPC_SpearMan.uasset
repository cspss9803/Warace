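; Spearman NPC Blueprint that specializes a parent NPC class with a spear (長槍) component.
; On BeginPlay it registers the spear as the static mesh needing the dissolve effect, then runs parent logic.
; It supplies weapon-specific transforms: the spear's hand_l socket location in RightHand bone space, suited to off-hand placement, and its 發射位置 socket as the world-space firing point.
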(event EventBeginPlay
  (Variables|Default|Set所有需要消散特效的靜態模型 (Utilities|Array|MakeArray (Variables|Default|Get長槍)))
  (|CallParentFunction))

(event Collision|EventActorBeginOverlap
  (params (OtherActor :type Actor%20Object%20Reference)))

(event EventTick
  (params (DeltaSeconds :type Float%20%28single-precision%29)))

(fn ConstructionScript
  (|CallParentFunction))

(fn FWeaponTransform
  (bind _長槍 (Variables|Default|Get長槍))
  (Utilities|IsValid _長槍
    (:Is%20Valid
      (return (Math|Transform|MakeTransform (.OutPosition (Class|SkinnedMeshComponent|TransformtoBoneSpace (Variables|Character|GetMesh) "RightHand" (.location (Transformation|GetSocketTransform _長槍 "hand_l" "RTS_World")) "0, 0, 0")) "0, 0, 0" "1.000000,1.000000,1.000000")))))

(fn FGet發射位置
  (bind _長槍 (Variables|Default|Get長槍))
  (Utilities|IsValid _長槍
    (:Is%20Valid
      (return (Transformation|GetSocketTransform _長槍 "發射位置" "RTS_World")))))