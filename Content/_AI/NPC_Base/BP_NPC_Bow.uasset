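; BP_NPC_Bow is an NPC blueprint for a bow wielder, adding bow-draw control to its parent's behavior.
; The 拉弓_Multicast (draw bow) event casts the ChildActor1 child actor to BP_W_Bow and forwards the draw or release flag to that weapon's 拉弓 function.
; BeginPlay and construction only call the parent, and the N_拉弓 function is an empty stub.
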(event Custom|拉弓_Multicast
  (params (是否拉弓 :type Boolean))
  (bind _childactor1 (Variables|Default|GetChildActor1))
  (bind _childactor (Variables|/Script/Engine.ChildActorComponent|GetChildActor _childactor1))
  (if 是否拉弓
    (bind _asbp_w_bow (Utilities|Casting|CastToBP_W_Bow _childactor))
    (Default|拉弓 _asbp_w_bow true)
    (else
      (bind _asbp_w_bow_2 (Utilities|Casting|CastToBP_W_Bow _childactor))
      (Default|拉弓 _asbp_w_bow_2 false))))

(event EventBeginPlay
  (|CallParentFunction))

(event Collision|EventActorBeginOverlap
  (params (OtherActor :type Actor%20Object%20Reference)))

(event EventTick
  (params (DeltaSeconds :type Float%20%28single-precision%29)))

(fn ConstructionScript
  (|CallParentFunction))

(fn N拉弓
  (params (是否拉弓 :type Boolean)))