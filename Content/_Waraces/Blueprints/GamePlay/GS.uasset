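; Game State for a two-player VR card battler that runs each match from character placement and buffs through battles and crystal destruction to game over.
; The replicated phase enum's OnRep launches each stage, with server countdowns driving timed transitions.
; Before fights, a FlipFlop alternates players' queued effects through delay-timed handlers, some letting opponents counter with Energy Shield or Purifying Light.
; Three battle wins cost the loser a crystal; losing all ends the game.
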(event Custom|效果展示
  (if (or (Utilities|Array|IsNotEmpty (Variables|/Game/_AI/NPC_Base/BP_NPC_Base.BP_NPC_Base_C|Get效果列表 (CallFunction|取得對戰角色))) (Utilities|Array|IsNotEmpty (Variables|/Game/_AI/NPC_Base/BP_NPC_Base.BP_NPC_Base_C|Get效果列表 (CallFunction|取得對戰角色 1))))
    ;[1 1 1] 輪流套用效果
    (bind _isa (Utilities|FlowControl|FlipFlop)
      (:A
        _)
      (:B
        _))
    (if (Utilities|Array|IsNotEmpty (Variables|/Game/_AI/NPC_Base/BP_NPC_Base.BP_NPC_Base_C|Get效果列表 (CallFunction|取得對戰角色 (select _isa 0 1))))
      (CallFunction|套用效果 (select _isa 0 1))
      (else
        (CallFunction|效果展示)))
    (else
      (Variables|Default|Set遊戲階段 "NewEnumerator4"))))

(event Custom|下個效果
  (params (需要隱藏展示效果的角色 :type BP%20NPC%20Base%20Object%20Reference))
  (Default|隱藏效果圖示 需要隱藏展示效果的角色)
  (Utilities|FlowControl|Delay 0.25)
  (CallFunction|效果展示))

(event Custom|套用效果
  (params (玩家序號 :type Integer))
  (bind _對戰角色 (CallFunction|取得對戰角色 玩家序號))
  (bind _效果列表 (Variables|/Game/_AI/NPC_Base/BP_NPC_Base.BP_NPC_Base_C|Get效果列表 _對戰角色))
  (bind _output (Utilities|Array|Get(acopy) _效果列表))
  (Variables|Default|Set目前要釋放的效果 "NewEnumerator4")
  (Default|更新效果 _對戰角色 _output)
  (Utilities|FlowControl|Sequence
    (:then_0
      (Utilities|FlowControl|Delay 0.3)
      (Utilities|Array|RemoveIndex _效果列表))
    (:then_1
      (Variables|Default|Set目前要釋放的效果 _output)
      (Utilities|FlowControl|Delay 0.25)
      (switch Utilities|FlowControl|Switch|SwitchonE_Buff (Variables|Default|Get目前要釋放的效果)
        (:NewEnumerator4
          (|展示效果-None _對戰角色))
        (:NewEnumerator0
          (|生命之石 _對戰角色))
        (:NewEnumerator1
          (|生命汲取 _對戰角色))
        (:NewEnumerator5
          (|生命藥水 _對戰角色))
        (:NewEnumerator6
          (|地獄召喚 _對戰角色))
        (:NewEnumerator7
          (|灼燒 _對戰角色))
        (:NewEnumerator8
          (|寒冰劍陣 _對戰角色))
        (:NewEnumerator9
          (|迅捷箭意 _對戰角色))
        (:NewEnumerator10
          (|命運之卡 _對戰角色))
        (:NewEnumerator11
          (|勇士之力 _對戰角色))
        (:NewEnumerator12
          (|海洋之石 _對戰角色))
        (:NewEnumerator13
          (|海洋的祝福 _對戰角色))
        (:NewEnumerator14
          (|能量之盾 _對戰角色))
        (:NewEnumerator15
          (|淨化之光 _對戰角色))
        (:NewEnumerator16
          (|焚身之怒 _對戰角色))
        (:NewEnumerator17
          (|迷幻星芒 _對戰角色))
        (:NewEnumerator18
          (|聖光 _對戰角色))
        (:NewEnumerator19
          (|聖翼庇護 _對戰角色))
        (:NewEnumerator20
          (|聖靈之盾 _對戰角色))
        (:NewEnumerator21
          (|隕石衝擊 _對戰角色))
        (:NewEnumerator22
          (|閃電雷擊 _對戰角色))
        (:NewEnumerator23
          (|魅惑 _對戰角色))
        (:NewEnumerator24
          (|魔力要水 _對戰角色))
        (:NewEnumerator25
          (|魔法權杖 _對戰角色))
        (:NewEnumerator26
          (|致命利刃 _對戰角色))
        (:NewEnumerator27
          (|鎧甲勇士 _對戰角色))
        (:NewEnumerator28
          (|妖精儀式 _對戰角色))
        (:NewEnumerator29
          (|奇襲 _對戰角色))
        (:NewEnumerator30
          (|皮糙肉厚 _對戰角色))
        (:NewEnumerator31
          (|戰吼 _對戰角色))
        (:NewEnumerator32
          (|寶石手套 _對戰角色))))))

(fn ConstructionScript)

(fn OnRep遊戲階段
  (switch Utilities|FlowControl|Switch|SwitchonE_GameStage (Variables|Default|Get遊戲階段)
    (:NewEnumerator1
      (|角色安排階段 3.0))
    (:NewEnumerator9
      (|等待角色放置完成階段 1.0))
    (:NewEnumerator2
      (|增益添加階段 3.0))
    (:NewEnumerator3
      (|對戰角色生成階段 1.0))
    (:NewEnumerator10
      (|效果展示階段))
    (:NewEnumerator4
      (|對戰階段))
    (:NewEnumerator5
      (|獲勝檢查階段 1.0))
    (:NewEnumerator7
      (|生命水晶破壞階段))
    (:NewEnumerator6
      (|重設 2.0))
    (:NewEnumerator8
      (|遊戲結束))))

(fn OnRep所有玩家的玩家狀態
  ;[1 1 1] 更新記分板
  (bind _returnvalue (Actor|GetActorOfClass "/Game/_Waraces/Scene_UIs/MainMap/PlayerList/Actor_3D_Widget_PlayerList.Actor_3D_Widget_PlayerList_C"))
  (Default|UpdatePlayerList _returnvalue))

(fn 取得對戰角色
  (params (玩家序號 :type Integer))
  (bind _asps (Utilities|Casting|CastToPS (Utilities|Array|Get(acopy) (Variables|Default|GetPlayerArray) 玩家序號)))
  (bind _asbp_npc_base (Utilities|Casting|CastToBP_NPC_Base (Variables|/Game/_Waraces/Blueprints/GamePlay/PS.PS_C|Get目前的對戰角色 _asps)))
  (return _asbp_npc_base))

(event Custom|啟動玩家端的計時器
  (params (要倒數的時間 :type Float%20%28double-precision%29) (伺服端計時器的啟動時間點 :type Float%20%28double-precision%29))
  (bind _returnvalue (Actor|GetActorOfClass "/Game/_Waraces/Scene_UIs/MainMap/Timer/Actor_3D_Widget_Timer.Actor_3D_Widget_Timer_C"))
  (Default|LaunchPlayerTimer _returnvalue 要倒數的時間 伺服端計時器的啟動時間點))

(event Custom|LaunchTimer
  (params (Time :type Float%20%28double-precision%29) (Only%20Launch%20Server%20Timer? :type Boolean))
  (if (Networking|IsServer)
    (CallFunction|LaunchServerTimer Time)
    (if (not Only%20Launch%20Server%20Timer?)
      (CallFunction|啟動玩家端的計時器 Time (Variables|Default|Get伺服器計時器啟動的時間點)))))

(event Custom|PlayerAmountChange
  (Variables|Default|Set所有玩家的玩家狀態 (Variables|Default|GetPlayerArray)))

(event Custom|ServerCountDown
  (bind _result (Math|Float|DecrementFloat (Variables|Default|Get伺服器的倒數計時時間))
    (:%20%20
      (if (not (> _result 0.0))
        (Utilities|Time|ClearandInvalidateTimerbyHandle (Variables|Default|Get伺服器計時器))
        (return)))))

(event Custom|LaunchServerTimer
  (params (Time :type Float%20%28double-precision%29))
  (Variables|Default|Set伺服器的倒數計時時間 Time)
  (Variables|Default|Set伺服器計時器啟動的時間點 (GameState|GetServerWorldTimeSeconds))
  (bind _returnvalue (Utilities|Time|SetTimerbyEvent (delegate Custom|ServerCountDown) 1.0 true))
  (Variables|Default|Set伺服器計時器 _returnvalue))