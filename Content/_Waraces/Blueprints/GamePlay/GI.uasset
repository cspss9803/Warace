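; Game instance for the VR game, handling level travel, LAN session hosting and joining, IP connection, quitting, and player data.
; Travel events mostly show status on the headset message UI.
; Init caches the player's profile, coins and unlocks from GUID-keyed requests, or fabricates them in developer mode.
; Match settlement awards randomized coins (reduced for losers), spawns the result actor and enables leaving; a helper spawns VR keyboards.
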(event Custom|IP%20連線
  (params (IP :type Text))
  (Development|ExecuteConsoleCommand (Utilities|String|ToString(Text) (Utilities|Text|FormatText "open {ip}" IP)) (Game|GetPlayerController 0)))

(event Custom|創建房間
  (params (頭顯訊息介面 :type WB%20HMD%20Start%20Object%20Reference) (房間名稱 :type String) (房間圖片 :type Integer))
  (bind _returnvalue (Utilities|String|TrimTrailing 房間名稱))
  (Default|顯示過場遮罩 頭顯訊息介面 "創建中...")
  (Utilities|FlowControl|Delay 1.0)
  (|AdvancedSession (Utilities|Array|MakeArray (Class|AdvancedSessionsLibrary|MakeLiteralSessionPropertyString (CallFunction|取得房間名稱Key) (select (Utilities|Array|IsEmpty _returnvalue) (Utilities|String|GetSubstring (Guid|ToString(Guid) (Guid|NewGuid)) 0 10) _returnvalue)) (Class|AdvancedSessionsLibrary|MakeLiteralSessionPropertyInt (CallFunction|取得房間圖片Key) (select (or (> 房間圖片 30) (< 房間圖片 0)) (Math|Random|RandomInteger 30) 房間圖片))) (Game|GetPlayerController 0) 10 0 true true false true true true false false false true false true
    (:OnSuccess
      (Game|OpenLevel(byObjectReference) "/Game/_Waraces/Maps/Map_Main.Map_Main" true "?Listen"))
    (:OnFailure
      (Default|隱藏過場遮罩 頭顯訊息介面 "創建時發生錯誤" 1.0))))

(event Custom|關閉遊戲
  (params (頭顯訊息介面 :type WB%20HMD%20Start%20Object%20Reference))
  (Default|顯示過場遮罩 頭顯訊息介面 "正在關閉...")
  (Utilities|FlowControl|Delay 1.0)
  (Game|QuitGame (Game|GetPlayerController 0) "Quit" false))

(event Custom|金幣結算
  (params (是否獲勝 :type Boolean) (獲勝結果生成位置 :type Transform))
  (bind _returnvalue (Class|KismetSystemLibrary|MakeLiteralInteger 100))
  (bind _returnvalue_2 (Math|Random|RandomInteger 26))
  (bind _returnvalue_3 (+ _returnvalue _returnvalue_2))
  (bind _returnvalue_4 (/ _returnvalue_3 10))
  (bind _returnvalue_5 (* _returnvalue_4 7))
  (bind _returnvalue_6 (select 是否獲勝 _returnvalue_3 _returnvalue_5))
  (if (Variables|Default|Get開發者模式)
    (Game|SpawnActorfromClass "/Game/_Waraces/Scene_UIs/MainMap/GameResult/BP_GameResult.BP_GameResult_C" 獲勝結果生成位置 "Undefined" 0 是否獲勝 _returnvalue_6 0)
    (Utilities|FlowControl|Delay 1.0 :!label _label)
    (bind _asvrpawn_main (Utilities|Casting|CastToVRPawn_Main (Game|Player|GetPlayerPawn 0)))
    (Default|顯示系統訊息 (Variables|/Game/_Waraces/Player/Blueprints/VR_Pawn_Base.VR_Pawn_Base_C|Get頭顯訊息介面 _asvrpawn_main) -1.0 "按下 A 回到主選單" false)
    (Default|允許離開 _asvrpawn_main)
    (else
      (bind (_原有金幣 _現有金幣 _錯誤) (Utilities|金幣增加 (Variables|Default|Get身份證) _returnvalue_6)
        (:增加成功
          (Game|SpawnActorfromClass "/Game/_Waraces/Scene_UIs/MainMap/GameResult/BP_GameResult.BP_GameResult_C" 獲勝結果生成位置 "Undefined" 0 是否獲勝 (- _現有金幣 _原有金幣) 0)
          (goto _label))
        (:發生錯誤
          (|金幣結算錯誤回報 _錯誤))))))

(event Custom|中斷連線
  (Game|OpenLevel(byObjectReference) "/Game/_Waraces/Maps/Map_Login.Map_Login"))

(event Custom|開始新手導覽
  (params (頭顯訊息介面 :type WB%20HMD%20Start%20Object%20Reference))
  (Default|顯示過場遮罩 頭顯訊息介面 "正在前往新手導覽...")
  (Utilities|FlowControl|Delay 1.0)
  (Game|OpenLevel(byObjectReference) "/Game/_Waraces/Maps/Map_Guide.Map_Guide"))

(event Custom|前往商城
  (params (頭顯訊息介面 :type WB%20HMD%20Start%20Object%20Reference))
  (Default|顯示過場遮罩 頭顯訊息介面 "正在前往商城...")
  (Utilities|FlowControl|Delay 1.0)
  (Game|OpenLevel(byObjectReference) "/Game/Store/Map_Store.Map_Store"))

(event Custom|用Session連線到房間
  (params (頭顯訊息介面 :type WB%20HMD%20Start%20Object%20Reference) (搜尋到的房間 :type Blueprint%20Session%20Result%20Structure))
  (Default|設定系統訊息 頭顯訊息介面 "連線中...")
  (|加入房間Session 搜尋到的房間
    (:OnSuccess
      (Default|設定系統訊息 頭顯訊息介面 "連線成功，正在加入房間"))
    (:OnFailure
      (Default|隱藏過場遮罩 頭顯訊息介面 "連線時發生錯誤" 1.0))))

(event EventInit
  (if (Variables|Default|Get開發者模式)
    (|設定開發者模式的玩家資料 1000 5.0 (|選擇要解鎖的角色 true false false false true false false false false true false false))
    (else
      (|如果已經登入)
      (bind (_玩家暱稱 _持有金幣 _擁有角色的解鎖狀態 _水晶攻擊特效的擁有與解鎖狀態 _傷害文字特效的擁有與解鎖狀態 _錯誤) (Utilities|取得玩家資料 (Variables|Default|Get身份證))
        (:資料取得成功
          (|儲存取得的資料 _玩家暱稱 _持有金幣 _擁有角色的解鎖狀態 _水晶攻擊特效的擁有與解鎖狀態 _傷害文字特效的擁有與解鎖狀態))
        (:發生錯誤
          (|錯誤回報 _錯誤))))))

(fn 生成虛擬鍵盤
  (params (要輸入文字的輸入框 :type Editable%20Text%20Object%20Reference) (覆蓋在輸入框上用來觸發輸入的按鈕 :type Button%20Object%20Reference) (是否要禁止空格字元? :type Boolean))
  (bind _returnvalue (Game|SpawnActorfromClass "/Game/_Waraces/Scene_UIs/StartMap/Keyboard/BP_Keyboard.BP_Keyboard_C" (Math|Transform|MakeTransform "80.000000,0.000000,80.000000" "-30.000000,0.000000,0.000000" "1.000000,1.000000,1.000000") "Undefined" (Game|GetPlayerController 0) 要輸入文字的輸入框 覆蓋在輸入框上用來觸發輸入的按鈕 是否要禁止空格字元? 0))
  (Utilities|FlowControl|Sequence
    (:then_0
      (if (not (Class|HeadMountedDisplayFunctionLibrary|IsHeadMountedDisplayEnabled))
        (Class|Widget|SetUserFocus 要輸入文字的輸入框 (Game|GetPlayerController 0))))
    (:then_1
      (return _returnvalue))))

(fn Debug生成角色解鎖狀態
  (params (要解鎖的角色 :type Set%20of%20E_NPC%20Enums :default "NewEnumerator0"))
  (bind _array (Utilities|Array|MakeArray "NewEnumerator1" "NewEnumerator2"))
  (bind _result (Utilities|Set|ToArray 要解鎖的角色))
  (for _array_element _result
    (if (not (or (Utilities|Enum|Equal(Enum) _array_element "NewEnumerator6") (Utilities|Enum|Equal(Enum) _array_element "NewEnumerator0")))
      (Utilities|Array|Add (LocalVariables|Get解鎖角色) (Utilities|Struct|MakeS_OwnedCharacterState _array_element _array _array _array "NewEnumerator1" "NewEnumerator1" "NewEnumerator1"))))
  (return (LocalVariables|Get解鎖角色)))