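; BP_AOE_OverTime_StonePillar is an AI attack area-of-effect variant that presents its hit as a stone pillar.
; It extends the parent's HitActor event, marked as one-time damage, by calling the parent logic and then a pillar-spawning custom event.
; That event attaches a rock particle emitter to the actor's root and plays a rubble sound at the actor's location.
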(event Custom|生成石柱
  (params (AttachToComponent :type Scene%20Component%20Object%20Reference))
  (Effects|SpawnEmitterAttached "/Game/_AI/NPC_Beast/VFX/AdvancedMagicFX11/Particles/P_ky_rock2.P_ky_rock2" AttachToComponent "None")
  (Audio|PlaySoundatLocation "/Game/_AI/NPC_Beast/Audio/碎石.碎石" (Transformation|GetActorLocation self) "0, 0, 0" 1.0 1.0 0.0 0 0 0 0))

(event EventBeginPlay
  (|CallParentFunction) ; This node is disabled and will not be called.\nDrag off pins to build functionality.
)

(event Collision|EventActorBeginOverlap
  (params (OtherActor :type Actor%20Object%20Reference))
  (|CallParentFunction OtherActor) ; This node is disabled and will not be called.\nDrag off pins to build functionality.
)

(event EventTick
  (params (DeltaSeconds :type Float%20%28single-precision%29))
  (|CallParentFunction DeltaSeconds) ; This node is disabled and will not be called.\nDrag off pins to build functionality.
)

(event EventHitActor
  (|CallParentFunction)
  (CallFunction|生成石柱 (Variables|Default|GetDefaultSceneRoot)))

(fn ConstructionScript
  (|CallParentFunction))