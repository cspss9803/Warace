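; Display actor for an NPC that builds its look from the NPC type: skeletal mesh, anim Blueprint and socketed weapons.
; On BeginPlay, a timeline drives a type-colored dissolve on body and weapon materials and Niagara effects.
; For the local player's own side, it creates a buff-list widget that turns toward the camera each Tick.
; It also refreshes the slot's info panel and computes a right-hand bone-space transform from the hammer's socket.
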(event Custom|更新資訊面板
  (bind _角色資訊面板介面 (Variables|/Game/_Waraces/Cards/Card_UIs/CardSlot/BP_CardSlot.BP_CardSlot_C|Get角色資訊面板介面 (Variables|Default|Get槽位))
    (:then
      (Default|更新屬性 _角色資訊面板介面))
    (:else)))

(event EventBeginPlay
  (bind _npc_種類 (Variables|Default|GetNPC%20種類))
  (bind _niagarasystemdissolving_sk (Variables|Default|GetNiagaraSystemDissolving_SK))
  (bind _mesh (Variables|Character|GetMesh))
  (bind _顏色 (CallFunction|取得NPC的顏色 _npc_種類))
  (bind _returnvalue (Math|Conversions|ToVector(LinearColor) _顏色))
  (Components|SkeletalMesh|SetSkeletalMeshAsset (Variables|Character|GetMesh) (CallFunction|取得NPC的骨骼模型 (Variables|Default|GetNPC%20種類)))
  (Class|SkeletalMeshComponent|SetAnimClass (Variables|Character|GetMesh) (CallFunction|取得NPC的動畫藍圖類別 (Variables|Default|GetNPC%20種類)))
  (|設定武器 (Variables|Default|GetNPC%20種類) (Variables|Character|GetMesh)
    (:execute
      (Utilities|FlowControl|Sequence
        (:then_0
          (if (and (CallFunction|此邏輯是否執行於該玩家的本地端上? (Variables|Default|Get玩家角色)) (Variables|Default|Get是否屬於我方))
            (Class|WidgetComponent|SetDrawSize (Variables|Default|Get效果列表介面) "(X=1500.000000,Y=300.000000)")
            (bind _returnvalue_2 (UserInterface|CreateWidget "/Game/_Waraces/Cards/Card_UIs/BuffList/WB_BuffList.WB_BuffList_C" 0 (Variables|Default|Get玩家角色) self))
            (bind _output_get (Variables|Default|Set效果列表容器 _returnvalue_2))
            (UserInterface|SetWidget (Variables|Default|Get效果列表介面) _output_get)
            (Utilities|FlowControl|Gate true) ; enters at Open
          ))
        (:then_1
          ;[1 1 1] Comment
          (Rendering|Material|SetVectorParameterValueonMaterials (Variables|Character|GetMesh) "Tint" _returnvalue)
          (Utilities|FlowControl|Sequence
            (:then_0
              (Rendering|Material|SetScalarParameterValueonMaterials _mesh "DissolvingAmount" 1.0)
              (Niagara|SetNiagaraVariable(Float) _niagarasystemdissolving_sk "DissolvingAmount" 1.0))
            (:then_1
              (Rendering|Material|SetVectorParameterValueonMaterials _mesh "DissolvingEdgeColor" _returnvalue)
              (Niagara|SetNiagaraVariable(LinearColor) _niagarasystemdissolving_sk "ParticleColor" _顏色))
            (:then_2
              (bind _tl_animation (Timeline|Timeline PlayFromStart)
                (:Update
                  (Rendering|Material|SetScalarParameterValueonMaterials (Variables|Character|GetMesh) "DissolvingAmount" _tl_animation)
                  (Niagara|SetNiagaraVariable(Float) (Variables|Default|GetNiagaraSystemDissolving_SK) "DissolvingAmount" _tl_animation)
                  (for _array_element (Variables|Default|Get武器)
                    (Rendering|Material|SetScalarParameterValueonMaterials _array_element "DissolvingAmount" _tl_animation)
                    (Niagara|SetNiagaraVariable(Float) (Variables|Default|GetNiagaraSystemDissolving_SM) "DissolvingAmount" _tl_animation)))))))))))

(event EventTick
  (params (DeltaSeconds :type Float%20%28single-precision%29))
  (Utilities|FlowControl|Gate true
    (:Exit
      (bind _asplayer_controller (Utilities|Casting|CastToPlayerController (Components|GetOwner)))
      (Transformation|SetWorldRotation (Variables|Default|Get效果列表介面) (Math|Rotator|FindLookatRotation (Transformation|GetWorldLocation (Variables|Default|Get效果列表介面)) (Camera|GetCameraLocation (Variables|/Script/Engine.PlayerController|GetPlayerCameraManager _asplayer_controller))) false false) ; 設定 Widget 的旋轉值，讓它面向鏡頭
    )))

(fn ConstructionScript)

(fn 取得NPC的骨骼模型
  (params (NPC :type E_NPC%20Enum :default "NewEnumerator0"))
  (switch Utilities|FlowControl|Switch|SwitchonE_NPC NPC
    (:NewEnumerator0
      (return 0))
    (:NewEnumerator4
      (return "/Game/_AI/NPC_Lava/Meshes/lava_Golem_low_1.lava_Golem_low_1"))
    (:NewEnumerator6
      (return "/Game/_AI/NPC_S_Goblin/Meshes/Low_Mesh_Rig.Low_Mesh_Rig"))
    (:NewEnumerator8
      (return "/Game/_AI/NPC_Goblin/Meshes/G_R_1.G_R_1"))
    (:NewEnumerator9
      (return "/Game/_AI/NPC_Forest/Meshes/R1.R1"))
    (:NewEnumerator10
      (return "/Game/_AI/NPC_Beast/Meshes/beast_RIG.beast_RIG"))
    (:NewEnumerator11
      (return "/Game/_AI/NPC_SpearMan/Meshes/Man_Rig.Man_Rig"))
    (:NewEnumerator12
      (return "/Game/_AI/NPC_Human/Meshes/Human_Rig.Human_Rig"))
    (:NewEnumerator13
      (return "/Game/_AI/NPC_Assassins/Meshes/ASSASSINS_RIG.ASSASSINS_RIG"))
    (:NewEnumerator14
      (return "/Game/_AI/NPC_Wolfman/Meshes/W_R.W_R"))
    (:NewEnumerator16
      (return "/Game/_AI/NPC_HeavyHammer/Meshes/beast-ii_Rig.beast-ii_Rig"))))

(fn 取得NPC的動畫藍圖類別
  (params (NPC :type E_NPC%20Enum :default "NewEnumerator0"))
  (switch Utilities|FlowControl|Switch|SwitchonE_NPC NPC
    (:NewEnumerator0
      (return 0))
    (:NewEnumerator4
      (return "/Game/_AI/NPC_Lava/ABP_Lava.ABP_Lava_C"))
    (:NewEnumerator6
      (return "/Game/_AI/NPC_S_Goblin/ABP_S_Goblin.ABP_S_Goblin_C"))
    (:NewEnumerator8
      (return "/Game/_AI/NPC_Goblin/ABP_Goblin.ABP_Goblin_C"))
    (:NewEnumerator9
      (return "/Game/_AI/NPC_Forest/ABP_R1.ABP_R1_C"))
    (:NewEnumerator10
      (return "/Game/_AI/NPC_Beast/ABP_beast.ABP_beast_C"))
    (:NewEnumerator11
      (return "/Game/_AI/NPC_SpearMan/ABP_SpearMan.ABP_SpearMan_C"))
    (:NewEnumerator12
      (return "/Game/_AI/NPC_Human/Animation/ABP_Human.ABP_Human_C"))
    (:NewEnumerator13
      (return "/Game/_AI/NPC_Assassins/ABP_Assassins.ABP_Assassins_C"))
    (:NewEnumerator14
      (return "/Game/_AI/NPC_Wolfman/ABP_Wolf.ABP_Wolf_C"))
    (:NewEnumerator16
      (return "/Game/_AI/NPC_HeavyHammer/ABP_HammerBeast.ABP_HammerBeast_C"))))

(fn GetHeavyhammerWeaponTransform
  (bind _鎚子 (Variables|Default|Get鎚子))
  (Utilities|IsValid _鎚子
    (:Is%20Valid
      (return (Math|Transform|MakeTransform (.OutPosition (Class|SkinnedMeshComponent|TransformtoBoneSpace (Variables|Character|GetMesh) "RightHand" (.location (Transformation|GetSocketTransform _鎚子 "hand_l" "RTS_World")) "0, 0, 0")) "0, 0, 0" "1.000000,1.000000,1.000000")))))