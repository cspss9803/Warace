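; Child AOE-over-time attack actor for a sword-light (劍光) strike, adding a slash visual to the inherited hit behavior.
; Its HitActor override, commented as one-time damage, runs the parent logic and then calls the half-moon swing event (發射半月揮擊).
; That event spawns the NS_Slash_CiAb_01 Niagara system attached to the root component with auto-destroy.
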(event Custom|發射半月揮擊
  (params (AttachToComponent :type Scene%20Component%20Object%20Reference))
  (Niagara|SpawnSystemAttached "/Game/_AI/NPC_Assassins/特效/NiagaraMagicalSlashes/Fx/Slashes/NS_Slash_CiAb_01.NS_Slash_CiAb_01" AttachToComponent "None" "0, 0, 0" "0, 0, 0" "KeepRelativeOffset" true))

(event EventBeginPlay
  (|CallParentFunction) ; This node is disabled and will not be called.\nDrag off pins to build functionality.
)

(event Collision|EventActorBeginOverlap
  (params (OtherActor :type Actor%20Object%20Reference))
  (|CallParentFunction OtherActor) ; This node is disabled and will not be called.\nDrag off pins to build functionality.
)

(event EventTick
  (params (DeltaSeconds :type Float%20%28single-precision%29))
  (|CallParentFunction DeltaSeconds) ; This node is disabled and will not be called.\nDrag off pins to build functionality.
)

(event EventHitActor
  (|CallParentFunction)
  (CallFunction|發射半月揮擊 (Variables|Default|GetDefaultSceneRoot)))

(fn ConstructionScript
  (|CallParentFunction))