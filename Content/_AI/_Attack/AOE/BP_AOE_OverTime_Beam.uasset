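; Beam variant of an over-time AOE attack actor for AI, inheriting its behaviour from a parent Blueprint.
; BeginPlay sets the 特效 (effect) particle component's template to 進階攻擊特效 (advanced attack effect), without calling the parent BeginPlay.
; Trigger, commented as continuous damage, only forwards to the parent, as does the construction script.
; Overlap and Tick events are disabled stubs.
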(event EventBeginPlay
  (Effects|Components|ParticleSystem|SetTemplate (Variables|Default|Get特效) (Variables|Default|Get進階攻擊_特效)))

(event Collision|EventActorBeginOverlap
  (params (OtherActor :type Actor%20Object%20Reference))
  (|CallParentFunction OtherActor) ; This node is disabled and will not be called.\nDrag off pins to build functionality.
)

(event EventTick
  (params (DeltaSeconds :type Float%20%28single-precision%29))
  (|CallParentFunction DeltaSeconds) ; This node is disabled and will not be called.\nDrag off pins to build functionality.
)

(event EventTrigger
  (|CallParentFunction))

(fn ConstructionScript
  (|CallParentFunction))