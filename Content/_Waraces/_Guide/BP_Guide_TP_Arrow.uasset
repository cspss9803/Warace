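; BP_Guide_TP_Arrow is a teleport destination marker in the VR guide tutorial, with an arrow widget and a trigger box.
; Every tick, a look-at rotation turns the arrow widget to face the player camera.
; When a VR_Pawn_Guide overlaps the box, it calls that pawn's teleport-arrival function (傳送到達目的地).
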(event OnComponentBeginOverlap(Box)
  (params (OverlappedComponent :type Primitive%20Component%20Object%20Reference) (OtherActor :type Actor%20Object%20Reference) (OtherComp :type Primitive%20Component%20Object%20Reference) (OtherBodyIndex :type Integer) (bFromSweep :type Boolean) (SweepResult :type Hit%20Result%20Structure%20%28by%20ref%29))
  (bind _asvr_pawn_guide (Utilities|Casting|CastToVR_Pawn_Guide OtherActor))
  (Default|傳送到達目的地 _asvr_pawn_guide))

(event EventTick
  (params (DeltaSeconds :type Float%20%28single-precision%29))
  (|角色資訊介面持續轉向玩家_2))

(fn ConstructionScript)