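; BP_Timer is a main-map countdown display that shows a WB_Timer widget through a widget component rotated each tick toward the local player's camera.
; LaunchPlayerTimer subtracts server time elapsed since the timer's launch, then starts a looping one-second Count timer to update the text.
; Count plays a sound at ten, animates the final seconds and clears at zero.
; SetBattleCount reuses the text to show the battle number.
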(event Custom|LaunchPlayerTimer
  (params (Time :type Float%20%28double-precision%29) (ServerTimerLaunchTimePoint :type Float%20%28double-precision%29))
  (Class|TextBlock|SetFont (Variables|/Game/_Waraces/Scene_UIs/MainMap/Timer/WB_Timer.WB_Timer_C|GetText_time (Variables|Default|GetWB_Timer)) (Utilities|Struct|MakeSlateFontInfo "/Engine/EngineFonts/Roboto.Roboto" 0 "(OutlineSize=0,bSeparateFillAlpha=False,bApplyOutlineToDropShadows=False,OutlineMaterial=None,OutlineColor=(R=0.000000,G=0.000000,B=0.000000,A=1.000000))" "Bold" 64 0 0.0))
  (bind _output_get (Variables|Default|Settime (- Time (- (GameState|GetServerWorldTimeSeconds (Game|GetGameState)) ServerTimerLaunchTimePoint)))) ; 把正確的倒數時間設定到計時器的倒數時間上
  (Variables|/Script/UMG.TextBlock|SetText (Variables|Default|GetText%20Time) (Utilities|Text|ToText(Integer) (Math|Float|Round _output_get)))
  (bind _returnvalue (Utilities|Time|SetTimerbyEvent (delegate Custom|Count) 1.0 true (- _output_get (Math|Float|Round _output_get)))) ; 啟動介面上的計時器  ( 每秒計時 )
  (Variables|Default|Settimer _returnvalue) ; 把計時器儲存起來\n以便後面在計時結束之後可以用來清除計時器
)

(event Custom|Count
  (bind _wb_timer (Variables|Default|GetWB_Timer))
  (bind _wb_timer_2 (Variables|Default|GetWB_Timer))
  (bind _wb_timer_3 (Variables|Default|GetWB_Timer))
  (bind _text_time (Variables|Default|GetText%20Time))
  (bind _result (Math|Float|DecrementFloat (Variables|Default|Gettime)) ; 秒數減少1
    (:%20%20
      (Utilities|FlowControl|Sequence
        (:then_0
          (if (<= (Math|Float|Round _result) 0) ; 判斷倒數是否結束 ( 有沒有計時到0秒了 )
            (Variables|/Script/UMG.TextBlock|SetText _text_time "0")
            (Utilities|Time|ClearandInvalidateTimerbyHandle (Variables|Default|Gettimer)) ; 清除計時器
            (Utilities|FlowControl|Delay 0.5)
            (Variables|/Script/UMG.TextBlock|SetText (Variables|/Game/_Waraces/Scene_UIs/MainMap/Timer/WB_Timer.WB_Timer_C|GetText_time (Variables|Default|GetWB_Timer)) "")
            (UserInterface|Animation|PlayAnimation _wb_timer (Variables|/Game/_Waraces/Scene_UIs/MainMap/Timer/WB_Timer.WB_Timer_C|GetAn_淡出放大 _wb_timer) 0.0 1 "Reverse" 1.0 false)
            (Class|TextBlock|SetFont (Variables|/Game/_Waraces/Scene_UIs/MainMap/Timer/WB_Timer.WB_Timer_C|GetText_time (Variables|Default|GetWB_Timer)) (Utilities|Struct|MakeSlateFontInfo "/Engine/EngineFonts/Roboto.Roboto" 0 "(OutlineSize=0,bSeparateFillAlpha=False,bApplyOutlineToDropShadows=False,OutlineMaterial=None,OutlineColor=(R=0.000000,G=0.000000,B=0.000000,A=1.000000))" "Bold" 24 0 0.0))
            (else
              (Variables|/Script/UMG.TextBlock|SetText _text_time (Utilities|Text|ToText(Integer) (Math|Float|Round _result))))))
        (:then_1
          (if (== (Math|Float|Round _result) 10)
            (Audio|PlaySound2D "/Game/_Waraces/Scene_UIs/MainMap/Timer/SW_Timer_CountDown10.SW_Timer_CountDown10" 1.0 1.0 0.0 0 0)
            (UserInterface|Animation|PlayAnimation _wb_timer_2 (Variables|/Game/_Waraces/Scene_UIs/MainMap/Timer/WB_Timer.WB_Timer_C|GetAn_淡出放大 _wb_timer_2) 0.0 1 "Forward" 1.0 false :!label _label)
            (elif (< (Math|Float|Round _result) 10)
              (goto _label)
              (else
                (Variables|/Script/UMG.Widget|SetRenderOpacity _wb_timer_3 1.0)
                (Class|TextBlock|SetFont (Variables|/Game/_Waraces/Scene_UIs/MainMap/Timer/WB_Timer.WB_Timer_C|GetText_time _wb_timer_3) (Utilities|Struct|MakeSlateFontInfo "/Engine/EngineFonts/Roboto.Roboto" 0 "(OutlineSize=0,bSeparateFillAlpha=False,bApplyOutlineToDropShadows=False,OutlineMaterial=None,OutlineColor=(R=0.000000,G=0.000000,B=0.000000,A=1.000000))" "Bold" 64 0 0.0))
                (Variables|/Script/UMG.Widget|SetRenderTransform _wb_timer_3 (Utilities|Struct|MakeWidgetTransform "(X=0.000000,Y=0.000000)" "(X=1.000000,Y=1.000000)" "(X=0.000000,Y=0.000000)" 0.0))))))))))

(event Custom|SetBattleCount
  (params (BattleCount :type Integer))
  (Variables|/Script/UMG.TextBlock|SetText (Variables|Default|GetText%20Time) (Utilities|Text|FormatText "第 {BattleCount} 場對決" BattleCount)))

(event Custom|開始轉向玩家
  (params (玩家控制器 :type Player%20Controller%20Object%20Reference))
  (Variables|Default|Set玩家控制器 玩家控制器)
  (Utilities|FlowControl|Gate true) ; enters at Open
)

(event EventBeginPlay
  (bind _aswb_timer (Utilities|Casting|CastToWB_Timer (UserInterface|GetWidget (Variables|Default|GetWidgetComponent_Timer))))
  (Variables|Default|SetText%20Time (Variables|/Game/_Waraces/Scene_UIs/MainMap/Timer/WB_Timer.WB_Timer_C|GetText_time _aswb_timer))
  (Variables|Default|SetWB_Timer _aswb_timer)
  (CallFunction|開始轉向玩家 (Game|GetPlayerController 0)))

(event EventTick
  (params (DeltaSeconds :type Float%20%28single-precision%29))
  (Utilities|FlowControl|Gate true
    (:Exit
      (bind _玩家控制器 (Variables|Default|Get玩家控制器)
        (:then
          (Transformation|SetWorldRotation (Variables|Default|GetWidgetComponent_Timer) (Math|Rotator|FindLookatRotation (Transformation|GetWorldLocation (Variables|Default|GetWidgetComponent_Timer)) (Camera|GetCameraLocation (Variables|/Script/Engine.PlayerController|GetPlayerCameraManager _玩家控制器))) false false) ; 設定 Widget 的旋轉值，讓它面向鏡頭
        )
        (:else)))))

(fn ConstructionScript)