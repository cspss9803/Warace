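; Start-map Blueprint that hosts the login/register screen, WB_Login_register, in a widget component.
; On BeginPlay it creates the widget, drawn at 1920x1080 if the player's own ID GUID is invalid, or shrunk to one pixel if valid, effectively hiding it.
; The 開啟登入面板 (open login panel) event restores full size and replaces the widget with a new one flagged as following a password change.
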(event Custom|開啟登入面板
  (bind _widgetcomponent_rename (Variables|Default|GetWidgetComponent_Rename))
  (Class|WidgetComponent|SetDrawSize _widgetcomponent_rename "(X=1920.000000,Y=1080.000000)")
  (bind _returnvalue (UserInterface|CreateWidget "/Game/_Waraces/Scene_UIs/StartMap/login_register/WB_Login_register.WB_Login_register_C" 0 true))
  (UserInterface|SetWidget _widgetcomponent_rename _returnvalue))

(event EventBeginPlay
  (bind _widgetcomponent_rename (Variables|Default|GetWidgetComponent_Rename))
  (if (not (Guid|IsValidGuid (CallFunction|取得自己的身分證)))
    (Class|WidgetComponent|SetDrawSize _widgetcomponent_rename "(X=1920.000000,Y=1080.000000)")
    (else
      (Class|WidgetComponent|SetDrawSize (Variables|Default|GetWidgetComponent_Rename) "(X=1.000000,Y=1.000000)")))
  (bind _returnvalue (UserInterface|CreateWidget "/Game/_Waraces/Scene_UIs/StartMap/login_register/WB_Login_register.WB_Login_register_C"))
  (UserInterface|SetWidget _widgetcomponent_rename _returnvalue))

(fn ConstructionScript)