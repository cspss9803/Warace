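; Base VR pawn that sets up headset play and lets both hands point at and click widgets.
; On BeginPlay it caches the HMD message widget, gives both widget interactors the player's virtual user index and random pointer IDs.
; If an HMD is enabled, it also sets Stage tracking origin, pixel density and the VR input mapping.
; Trigger inputs press and release pointer clicks with debug color feedback, while hover changes play per-hand haptics.
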(event OnHoveredWidgetChanged(介面互動器-右)
  (params (WidgetComponent :type Widget%20Component%20Object%20Reference) (PreviousWidgetComponent :type Widget%20Component%20Object%20Reference))
  (bind _asplayer_controller (Utilities|Casting|CastToPlayerController (Pawn|GetController)))
  (Class|PlayerController|PlayHapticEffect _asplayer_controller "/Game/_Waraces/Player/Haptic_Effect/HapticEffect_Hover.HapticEffect_Hover" "Right" 1.0 false) ; 發出輕震動
)

(event OnHoveredWidgetChanged(介面互動器-左)
  (params (WidgetComponent :type Widget%20Component%20Object%20Reference) (PreviousWidgetComponent :type Widget%20Component%20Object%20Reference))
  (bind _asplayer_controller (Utilities|Casting|CastToPlayerController (Pawn|GetController)))
  (Class|PlayerController|PlayHapticEffect _asplayer_controller "/Game/_Waraces/Player/Haptic_Effect/HapticEffect_Hover.HapticEffect_Hover" "Left" 1.0 false) ; 發出輕震動
)

(event Input|EnhancedActionEvents|EnhancedInputActionIA_Click_Right
  (params (ActionValue :type Boolean) (ElapsedSeconds :type Float%20%28double-precision%29) (TriggeredSeconds :type Float%20%28double-precision%29) (InputAction :type Input%20Action%20Object%20Reference :default "/Game/_Waraces/Player/Inputs/IA_Click_Right.IA_Click_Right"))
  (bind _介面互動器_右 (Variables|Default|Get介面互動器-右))
  (:Started
    (Class|WidgetInteractionComponent|PressPointerKey _介面互動器_右 "LeftMouseButton")
    (Variables|/Script/UMG.WidgetInteractionComponent|SetDebugColor _介面互動器_右 (Variables|Default|Get顏色-介面互動器-按下)))
  (:Completed
    (Class|WidgetInteractionComponent|ReleasePointerKey _介面互動器_右 "LeftMouseButton")
    (Variables|/Script/UMG.WidgetInteractionComponent|SetDebugColor _介面互動器_右 (Variables|Default|Get顏色-介面互動器-鬆開))))

(event Input|EnhancedActionEvents|EnhancedInputActionIA_Click_Left
  (params (ActionValue :type Boolean) (ElapsedSeconds :type Float%20%28double-precision%29) (TriggeredSeconds :type Float%20%28double-precision%29) (InputAction :type Input%20Action%20Object%20Reference :default "/Game/_Waraces/Player/Inputs/IA_Click_Left.IA_Click_Left"))
  (bind _介面互動器_左 (Variables|Default|Get介面互動器-左))
  (:Triggered
    (Class|WidgetInteractionComponent|PressPointerKey _介面互動器_左 "LeftMouseButton")
    (Variables|/Script/UMG.WidgetInteractionComponent|SetDebugColor _介面互動器_左 (Variables|Default|Get顏色-介面互動器-按下)))
  (:Completed
    (Class|WidgetInteractionComponent|ReleasePointerKey _介面互動器_左 "LeftMouseButton")
    (Variables|/Script/UMG.WidgetInteractionComponent|SetDebugColor _介面互動器_左 (Variables|Default|Get顏色-介面互動器-鬆開))))

(event EventBeginPlay
  (Utilities|FlowControl|Sequence
    (:then_0
      (bind _aswb_hmd (Utilities|Casting|CastToWB_HMD (UserInterface|GetWidget (Variables|Default|Get頭顯訊息介面%28WidgetComponent%29))))
      (Variables|Default|Set頭顯訊息介面 _aswb_hmd))
    (:then_1
      (|設定介面控制器的虛擬使用者序號)
      (Utilities|是否啟用了虛擬實境設備?
        (:已啟用
          (|設定VR裝置追蹤位置的基準點)
          (|設定顯示器的像素密度)
          (|設定映射輸入))))))

(fn ConstructionScript)