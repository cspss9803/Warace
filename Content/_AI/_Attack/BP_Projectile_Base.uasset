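; BP_Projectile_Base is an AI attack projectile that flies toward a target and reports hits on NPCs.
; Construction applies speed, gravity and optional homing on the target's root component.
; BeginPlay ignores the instigator (or owner) while moving, aims velocity at the target and stores the owner.
; Box overlap with a non-owner NPC calls OnProjectileImpact, then spawns Niagara or Cascade effects, which lead into sound and self-destruction.
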(event OnComponentBeginOverlap(BoxCollision)
  (params (OverlappedComponent :type Primitive%20Component%20Object%20Reference) (OtherActor :type Actor%20Object%20Reference) (OtherComp :type Primitive%20Component%20Object%20Reference) (OtherBodyIndex :type Integer) (bFromSweep :type Boolean) (SweepResult :type Hit%20Result%20Structure%20%28by%20ref%29))
  (bind _location (Collision|BreakHitResult SweepResult))
  (Utilities|FlowControl|Sequence
    (:then_0
      (bind _asbp_npc_base (Utilities|Casting|CastToBP_NPC_Base OtherActor))
      (if (and (!= _asbp_npc_base (Variables|Default|Get擁有者)) (Actor|ActorHasTag _asbp_npc_base "NPC"))
        (Default|CallOnProjectileImpact _asbp_npc_base SweepResult)
        (bind _arrow (Variables|Components|GetArrow)
          (:then
            (Utilities|FlowControl|Sequence
              (:then_0
                (bind _impact_effect (Variables|Effects|GetImpact%20Effect)
                  (:then
                    (Niagara|SpawnSystematLocation _impact_effect _location (Transformation|GetWorldRotation _arrow)))
                  (:else)))
              (:then_1
                (bind _emitter_template (Variables|Default|GetEmitter%20Template)
                  (:then
                    (Effects|SpawnEmitteratLocation _emitter_template _location (Transformation|GetWorldRotation _arrow)))
                  (:else))))
            (Audio|PlaySoundatLocation (Variables|Sounds|GetSound) _location "0, 0, 0" 1.0 1.0 0.0 0 0 0 0)
            (Actor|DestroyActor))
          (:else))))))

(event Custom|RotateToTarget
  (Variables|/Script/Engine.MovementComponent|SetVelocity (Variables|Components|GetProjectileMovement) (* (Math|Vector|GetUnitDirection(Vector) (Transformation|GetActorLocation) (Transformation|GetActorLocation (Variables|Target|GetTarget))) (Variables|ProjectileSetting|GetSpeed))))

(event EventBeginPlay
  (bind _returnvalue (Game|GetInstigator))
  (bind _returnvalue_2 (Components|GetOwner))
  (Collision|IgnoreActorwhenMoving (Variables|Components|GetBoxCollision) (select (Utilities|IsValid _returnvalue) _returnvalue _returnvalue_2) true) ; 忽略生成的玩家
  (Variables|Target|GetTarget
    (:then
      (CallFunction|RotatetoTarget)
      (Variables|Default|Set擁有者 _returnvalue_2))
    (:else)))

(fn ConstructionScript
  (bind _projectilemovement (Variables|Components|GetProjectileMovement))
  (bind _speed (Variables|ProjectileSetting|GetSpeed))
  (Variables|/Script/Engine.ProjectileMovementComponent|SetInitialSpeed _projectilemovement _speed)
  (Variables|/Script/Engine.ProjectileMovementComponent|SetMaxSpeed _projectilemovement _speed)
  (Variables|/Script/Engine.ProjectileMovementComponent|SetProjectileGravityScale _projectilemovement (Variables|ProjectileSetting|GetGravity))
  (Variables|Target|GetTarget
    (:then
      (if (Variables|ProjectileSetting|GetIsHoming) ; Homing就是角色移動會追蹤
        (Variables|/Script/Engine.ProjectileMovementComponent|SetbIsHomingProjectile _projectilemovement true)
        (Variables|/Script/Engine.ProjectileMovementComponent|SetHomingTargetComponent _projectilemovement (Variables|/Script/Engine.Actor|GetRootComponent (Variables|Target|GetTarget))) ; 對應的目標會是場景組件
      ))
    (:else)))