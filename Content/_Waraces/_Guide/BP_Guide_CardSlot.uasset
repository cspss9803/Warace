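; BP_Guide_CardSlot is a numbered character slot actor for the Guide, holding a displayed character and its world-placed UI.
; On BeginPlay it creates info panel, slot and upright interaction button widgets, assigning each to a WidgetComponent.
; The slot widget receives the actor and info panel, and the button receives the slot widget.
; Events unlock slot interaction, flag the first summon as done, and update or hide the info panel.
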(event Custom|允許互動角色槽位
  (Variables|/Game/_Waraces/_Guide/WB_Guide_CardSlot.WB_Guide_CardSlot_C|Set是否允許互動槽位? (Variables|Default|Get角色槽位介面) true))

(event Custom|完成首次角色召喚
  (Variables|/Game/_Waraces/_Guide/WB_Guide_CardSlot.WB_Guide_CardSlot_C|Set是否完成首次角色召喚? (Variables|Default|Get角色槽位介面) true))

(event Custom|更新角色資訊面版
  (Default|更新資訊 (Variables|Default|Get角色資訊面板介面) (Variables|Default|Get目前生成在槽位上的展示角色)))

(event Custom|隱藏資訊面板
  (Default|隱藏資訊面板 (Variables|Default|Get角色資訊面板介面)))

(event EventBeginPlay
  (|設定角色資訊面板介面)
  (|設定角色槽位介面)
  (|設定槽位直立互動區))

(fn ConstructionScript)