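; BP_Character_Board is an in-world board on the main map that displays the versus character panel for the Red and Blue teams.
; The 儲存PlayerState event scans the GameState's PlayerArray to store team PlayerStates, returning after the first Red or Blue match.
; Once both PSRed and PSBlue are valid, it creates WB_Character_Board with them and assigns it to its Widget component.
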(event Custom|儲存PlayerState
  (|將雙方陣營的PlayerState存起來)
  (if (and (Utilities|IsValid (Variables|Default|GetPS_Red)) (Utilities|IsValid (Variables|Default|GetPS_Blue)))
    (bind _returnvalue (UserInterface|CreateWidget "/Game/_Waraces/Scene_UIs/MainMap/CharacterBoard/WB_Character_Board.WB_Character_Board_C" 0 (Variables|Default|GetPS_Red) (Variables|Default|GetPS_Blue)))
    (bind _output_get (Variables|Default|Set對戰角色面板 _returnvalue))
    (UserInterface|SetWidget (Variables|Default|GetWidget) _output_get)))

(fn ConstructionScript)