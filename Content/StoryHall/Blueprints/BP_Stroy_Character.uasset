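; Story Hall character that appears as a stone figure with a story widget, configured per character type.
; BeginPlay dresses an outer stone mesh and an inner model with matching skeleton, AnimBP and socketed weapons, tinting dissolve effects by character color.
; A VRPawn_Story entering the one-shot trigger box runs a timeline driving material and Niagara dissolve on stone body and weapons.
; When it finishes, the inner model's animation unpauses and the widget allows story viewing.
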(event OnComponentBeginOverlap(Box)
  (params (OverlappedComponent :type Primitive%20Component%20Object%20Reference) (OtherActor :type Actor%20Object%20Reference) (OtherComp :type Primitive%20Component%20Object%20Reference) (OtherBodyIndex :type Integer) (bFromSweep :type Boolean) (SweepResult :type Hit%20Result%20Structure%20%28by%20ref%29))
  (Utilities|Casting|CastToVRPawn_Story OtherActor)
  (CallFunction|消散進場)
  (Components|DestroyComponent (Variables|Default|GetBox)))

(event Custom|消散進場
  (|隱形)
  (bind _newtrack_0 (Timeline|Timeline PlayFromStart)
    (:Update
      (Rendering|Material|SetScalarParameterValueonMaterials (Variables|Character|GetMesh) "DissolvingAmount" _newtrack_0)
      (Niagara|SetNiagaraVariable(Float) (Variables|Default|GetSkeletalMeshDissolving) "DissolvingAmount" _newtrack_0)
      (for _array_element (Variables|Default|Get石頭武器)
        (Rendering|Material|SetScalarParameterValueonMaterials _array_element "DissolvingAmount" _newtrack_0)
        (Niagara|SetNiagaraVariable(Float) (Variables|Default|Get靜態模型消散特效) "DissolvingAmount" _newtrack_0)))
    (:Finished
      (Variables|/Script/Engine.SkeletalMeshComponent|SetbPauseAnims (Variables|Default|Get內部骨骼模型) false)
      (Default|允許查看角色故事 (Variables|Default|GetWB%20Story)))))

(event EventBeginPlay
  (bind _returnvalue (UserInterface|CreateWidget "/Game/StoryHall/Blueprints/WB_Story.WB_Story_C" 0 (Variables|Default|Get角色種類)))
  (bind _output_get (Variables|Default|SetWB%20Story _returnvalue))
  (UserInterface|SetWidget (Variables|Default|GetWidget) _output_get)
  (Components|SkeletalMesh|SetSkeletalMeshAsset (Variables|Default|Get內部骨骼模型) (CallFunction|取得骨架模型 (Variables|Default|Get角色種類)))
  (Rendering|Material|SetMaterial (Variables|Character|GetMesh) 0 "/Game/StoryHall/MI_Stone_Character.MI_Stone_Character")
  (Class|SkeletalMeshComponent|SetAnimClass (Variables|Character|GetMesh) (CallFunction|取得ABP (Variables|Default|Get角色種類)))
  (|設定石頭武器 (Variables|Default|Get角色種類) (Variables|Character|GetMesh)
    (:execute
      (|設定武器 (Variables|Default|Get角色種類) (Variables|Default|Get內部骨骼模型)
        (:execute
          (|設定消散顏色)
          (Utilities|FlowControl|Sequence
            (:then_0
              (if (Utilities|Enum|Equal(Enum) (Variables|Default|Get角色種類) "NewEnumerator6")
                (Components|DestroyComponent (Variables|Default|GetWidget))))
            (:then_1
              (if (Utilities|Enum|Equal(Enum) (Variables|Default|Get角色種類) "NewEnumerator11")
                (Transformation|SetRelativeLocationAndRotation (Variables|Character|GetMesh) "-25.000000,0.000000,-90.000000" "0.000000,-140.000000,0.000000" false false)))
            (:then_2
              (if (Utilities|Enum|Equal(Enum) (Variables|Default|Get角色種類) "NewEnumerator14")
                (Transformation|SetRelativeLocation (Variables|Character|GetMesh) "-25.000000,0.000000,-90.000000" false false)))))))))

(fn ConstructionScript)

(fn 取得骨架模型
  (params (角色種類 :type E_NPC%20Enum :default "NewEnumerator0"))
  (switch Utilities|FlowControl|Switch|SwitchonE_NPC 角色種類
    (:NewEnumerator0
      (return 0))
    (:NewEnumerator4
      (return "/Game/_AI/NPC_Lava/Meshes/SK_Lava_Story.SK_Lava_Story"))
    (:NewEnumerator6
      (return "/Game/_AI/NPC_S_Goblin/Meshes/Low_Mesh_Rig.Low_Mesh_Rig"))
    (:NewEnumerator8
      (return "/Game/_AI/NPC_Goblin/Meshes/G_R_1.G_R_1"))
    (:NewEnumerator9
      (return "/Game/_AI/NPC_Forest/Meshes/R1.R1"))
    (:NewEnumerator10
      (return "/Game/_AI/NPC_Beast/Meshes/beast_RIG.beast_RIG"))
    (:NewEnumerator11
      (return "/Game/_AI/NPC_SpearMan/Meshes/Man_Rig.Man_Rig"))
    (:NewEnumerator12
      (return "/Game/_AI/NPC_Human/Meshes/Human_Rig.Human_Rig"))
    (:NewEnumerator13
      (return "/Game/_AI/NPC_Assassins/Meshes/ASSASSINS_RIG.ASSASSINS_RIG"))
    (:NewEnumerator14
      (return "/Game/_AI/NPC_Wolfman/Meshes/W_R.W_R"))
    (:NewEnumerator16
      (return "/Game/_AI/NPC_HeavyHammer/Meshes/beast-ii_Rig.beast-ii_Rig"))))

(fn 取得ABP
  (params (角色種類 :type E_NPC%20Enum :default "NewEnumerator0"))
  (switch Utilities|FlowControl|Switch|SwitchonE_NPC 角色種類
    (:NewEnumerator0
      (return 0))
    (:NewEnumerator4
      (return "/Game/_AI/NPC_Lava/ABP_Lava.ABP_Lava_C"))
    (:NewEnumerator6
      (return "/Game/_AI/NPC_S_Goblin/ABP_S_Goblin.ABP_S_Goblin_C"))
    (:NewEnumerator8
      (return "/Game/_AI/NPC_Goblin/ABP_Goblin.ABP_Goblin_C"))
    (:NewEnumerator9
      (return "/Game/_AI/NPC_Forest/ABP_R1.ABP_R1_C"))
    (:NewEnumerator10
      (return "/Game/_AI/NPC_Beast/ABP_beast.ABP_beast_C"))
    (:NewEnumerator11
      (return "/Game/_AI/NPC_SpearMan/ABP_SpearMan.ABP_SpearMan_C"))
    (:NewEnumerator12
      (return "/Game/_AI/NPC_Human/Animation/ABP_Human.ABP_Human_C"))
    (:NewEnumerator13
      (return "/Game/_AI/NPC_Assassins/ABP_Assassins.ABP_Assassins_C"))
    (:NewEnumerator14
      (return "/Game/_AI/NPC_Wolfman/ABP_Wolf.ABP_Wolf_C"))
    (:NewEnumerator16
      (return "/Game/_AI/NPC_HeavyHammer/ABP_HammerBeast.ABP_HammerBeast_C"))))

(fn GetHeavyhammerWeaponTransform
  (bind _mesh (Variables|Character|GetMesh))
  (bind _鎚子 (Variables|Default|Get鎚子))
  (bind _returnvalue (Transformation|GetSocketTransform _鎚子 "hand_l" "RTS_World"))
  (bind (_outposition _outrotation) (Class|SkinnedMeshComponent|TransformtoBoneSpace _mesh "RightHand" (.location _returnvalue) "0, 0, 0"))
  (Utilities|IsValid _鎚子
    (:Is%20Valid
      (return (Math|Transform|MakeTransform _outposition _outrotation "1.000000,1.000000,1.000000")))))