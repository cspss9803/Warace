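; Rain-of-arrows variant of an area-of-effect-over-time attack, adding the arrow rain visuals and audio to its parent's hit behavior.
; On HitActor it runs the parent logic, then calls the 召喚箭雨 (summon arrow rain) event.
; That event spawns an auto-destroying effect system attached slightly above the root component and plays the arrow rain sound at the actor's location.
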(event Custom|召喚箭雨
  (params (AttachToComponent :type Scene%20Component%20Object%20Reference))
  (Niagara|SpawnSystemAttached (Variables|Default|Get進階攻擊_特效) AttachToComponent "None" "0.000000,0.000000,50.000000" "0, 0, 0" "KeepRelativeOffset" true)
  (Audio|PlaySoundatLocation "/Game/_AI/NPC_Bow/Audio/箭雨音效.箭雨音效" (Transformation|GetActorLocation self) "0, 0, 0" 1.0 1.0 0.0 0 0 0 0))

(event EventBeginPlay
  (|CallParentFunction) ; This node is disabled and will not be called.\nDrag off pins to build functionality.
)

(event Collision|EventActorBeginOverlap
  (params (OtherActor :type Actor%20Object%20Reference))
  (|CallParentFunction OtherActor) ; This node is disabled and will not be called.\nDrag off pins to build functionality.
)

(event EventTick
  (params (DeltaSeconds :type Float%20%28single-precision%29))
  (|CallParentFunction DeltaSeconds) ; This node is disabled and will not be called.\nDrag off pins to build functionality.
)

(event EventHitActor
  (|CallParentFunction)
  (CallFunction|召喚箭雨 (Variables|Default|GetDefaultSceneRoot)))

(fn ConstructionScript
  (|CallParentFunction))