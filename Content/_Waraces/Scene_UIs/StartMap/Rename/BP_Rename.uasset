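; BP_Rename is an actor that hosts the player rename UI through a widget component, in the StartMap UI folder.
; On BeginPlay it reads PlayerName from the GI game instance and sizes the component to full HD if the name is empty, or shrinks it to one pixel otherwise.
; It then creates WB_Rename with a reference back to itself and assigns it to the component in either case.
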(event EventBeginPlay
  (bind _widgetcomponent_rename (Variables|Default|GetWidgetComponent_Rename))
  (bind _asgi (Utilities|Casting|CastToGI (Game|GetGameInstance)))
  (if (Utilities|Text|TextIsEmpty (Variables|/Game/_Waraces/Blueprints/GamePlay/GI.GI_C|GetPlayerName _asgi))
    (Class|WidgetComponent|SetDrawSize _widgetcomponent_rename "(X=1920.000000,Y=1080.000000)")
    (else
      (Class|WidgetComponent|SetDrawSize (Variables|Default|GetWidgetComponent_Rename) "(X=1.000000,Y=1.000000)")))
  (bind _returnvalue (UserInterface|CreateWidget "/Game/_Waraces/Scene_UIs/StartMap/Rename/WB_Rename.WB_Rename_C" 0 self))
  (UserInterface|SetWidget _widgetcomponent_rename _returnvalue))

(fn ConstructionScript)