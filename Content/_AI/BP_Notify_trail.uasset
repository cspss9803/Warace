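; Trail anim notify that picks the particle system for an NPC's weapon attack trail at runtime.
; OverridePSTemplate casts the mesh owner to BP_NPC_Base, switches on its character type (角色種類), then reads the normal-attack effect from the matching subclass.
; Only Heavy Hammer also checks attack type (攻擊類型), choosing between its normal and advanced effects.
; Spear Man, Tauren, Fairy, Stick and Sickle always use their normal-attack trail.
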(fn OverridePSTemplate
  (params (MeshComp :type Skeletal%20Mesh%20Component%20Object%20Reference) (Animation :type Anim%20Sequence%20Base%20Object%20Reference))
  (bind _returnvalue (Components|GetOwner MeshComp))
  (LocalVariables|SetGet%20Owner _returnvalue)
  (bind _asbp_npc_base (Utilities|Casting|CastToBP_NPC_Base _returnvalue))
  (switch Utilities|FlowControl|Switch|SwitchonE_NPC (Variables|/Game/_AI/NPC_Base/BP_NPC_Base.BP_NPC_Base_C|Get角色種類 _asbp_npc_base)
    (:NewEnumerator11
      (bind _asbp_npc_spear_man (Utilities|Casting|CastToBP_NPC_SpearMan (LocalVariables|GetGet%20Owner)))
      (LocalVariables|SetParticleSystem (Variables|/Game/_AI/NPC_Base/BP_NPC_SpearMan.BP_NPC_SpearMan_C|Get普通攻擊_Color _asbp_npc_spear_man)))
    (:NewEnumerator16
      (bind _asbp_npc_hammer_beast (Utilities|Casting|CastToBP_NPC_HammerBeast (LocalVariables|GetGet%20Owner)))
      (switch Utilities|FlowControl|Switch|SwitchonE_AttackData (Variables|/Game/_AI/NPC_Base/BP_NPC_Base.BP_NPC_Base_C|Get攻擊類型 _asbp_npc_base)
        (:NewEnumerator0
          (LocalVariables|SetParticleSystem (Variables|/Game/_AI/NPC_Base/BP_NPC_HammerBeast.BP_NPC_HammerBeast_C|Get普通攻擊_特效 _asbp_npc_hammer_beast)))
        (:NewEnumerator1
          (LocalVariables|SetParticleSystem (Variables|/Game/_AI/NPC_Base/BP_NPC_HammerBeast.BP_NPC_HammerBeast_C|Get進階攻擊_特效 _asbp_npc_hammer_beast)))))
    (:NewEnumerator18
      (bind _asbp_npc_tauren (Utilities|Casting|CastToBP_NPC_Tauren (LocalVariables|GetGet%20Owner)))
      (LocalVariables|SetParticleSystem (Variables|/Game/_AI/NPC_Base/BP_NPC_Tauren.BP_NPC_Tauren_C|Get普通攻擊_Color _asbp_npc_tauren)))
    (:NewEnumerator19
      (bind _asbp_npc_fairy (Utilities|Casting|CastToBP_NPC_Fairy (LocalVariables|GetGet%20Owner)))
      (LocalVariables|SetParticleSystem (Variables|/Game/_AI/NPC_Base/BP_NPC_Fairy.BP_NPC_Fairy_C|Get普通攻擊_特效 _asbp_npc_fairy)))
    (:NewEnumerator20
      (bind _asbp_npc_stick (Utilities|Casting|CastToBP_NPC_Stick (LocalVariables|GetGet%20Owner)))
      (LocalVariables|SetParticleSystem (Variables|/Game/_AI/NPC_Base/BP_NPC_Stick.BP_NPC_Stick_C|Get普通攻擊_特效 _asbp_npc_stick)))
    (:NewEnumerator21
      (bind _asbp_npc_sickle (Utilities|Casting|CastToBP_NPC_Sickle (LocalVariables|GetGet%20Owner)))
      (LocalVariables|SetParticleSystem (Variables|/Game/_AI/NPC_Base/BP_NPC_Sickle.BP_NPC_Sickle_C|Get普通攻擊_特效 _asbp_npc_sickle))))
  (return (LocalVariables|GetParticleSystem)))