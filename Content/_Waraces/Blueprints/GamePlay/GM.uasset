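; Game mode for a two-player VR card battle that admits players, makes later joiners spectators and draws random cards.
; PostLogin requests each controller's saved GUID; newcomers get a new one, though returning IDs have no handler.
; Players receive randomly ordered Red/Blue teams, a pawn and one life crystal, and two readies advance the game phase.
; Card draws pick random DataTable rows, rerolling excluded results.
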(event Custom|檢查身分證
  (params (身份證 :type Guid%20Structure) (玩家控制器 :type PC%20Object%20Reference))
  (|身份? 身份證
    (:新加入者
      (|玩家數量是否額滿?
        (:滿了
          (|加入到觀眾名單_成為觀眾 玩家控制器)
          (CallFunction|創建觀眾角色 玩家控制器)
          (|從待檢查身份的名單上剔除 玩家控制器 :!label _label)
          (Default|讓計時介面開始面向玩家 玩家控制器))
        (:未滿
          (Utilities|加入到玩家名單成為玩家 玩家控制器 (CallFunction|生成身份證))
          (Utilities|FlowControl|Sequence
            (:then_0
              (goto _label))
            (:then_1
              (CallFunction|創建玩家角色與生命水晶並設定陣營 玩家控制器)
              (|更新玩家列表介面))))))))

(event Custom|玩家準備完成
  (bind _result (Math|Integer|IncrementInt (Variables|Default|Get完成準備的玩家數量))
    (:%20%20
      (if (== _result 2) ; 是否雙方玩家都準備好了?
        (|進入對戰角色安排階段)
        (|儲存敵方的PS)))))

(event EventOnLogout
  (params (ExitingController :type Controller%20Object%20Reference))
  (bind _aspc (Utilities|Casting|CastToPC ExitingController))
  (|離開者的身份? _aspc
    (:身份未驗證者
      (Utilities|Array|RemoveItem (Variables|Default|Get等待身份檢查列表) _aspc))))

(event EventPostLogin
  (params (NewPlayer :type Player%20Controller%20Object%20Reference))
  (bind _aspc (Utilities|Casting|CastToPC NewPlayer))
  (Utilities|Array|Add (Variables|Default|Get等待身份檢查列表) _aspc)
  (Default|取得身份證 _aspc))

(fn ConstructionScript
  (bind _陣營分配列表 (Variables|Default|Get陣營分配列表))
  (bind _陣營分配列表_2 (Variables|Default|Get陣營分配列表))
  (switch int (Math|Random|RandomInteger 2)
    (:0
      (Utilities|Array|Add _陣營分配列表_2 "NewEnumerator1")
      (Utilities|Array|Add _陣營分配列表_2 "NewEnumerator2"))
    (:1
      (Utilities|Array|Add _陣營分配列表 "NewEnumerator2")
      (Utilities|Array|Add _陣營分配列表 "NewEnumerator1"))))

(fn 創建玩家角色與生命水晶並設定陣營
  (params (玩家控制器 :type PC%20Object%20Reference%20%28by%20ref%29))
  (bind _returnvalue (Class|KismetSystemLibrary|MakeLiteralInteger 2))
  (for (_array_element _array_index) (Variables|Default|Get玩家名單)
    (if (== 玩家控制器 (.玩家控制器 (Utilities|Struct|BreakStruct_PlayerList _array_element)))
      (LocalVariables|Set玩家編號 _array_index)
      (LocalVariables|Set玩家陣營 (Utilities|Array|Get(acopy) (Variables|Default|Get陣營分配列表) (LocalVariables|Get玩家編號)))
      (switch int (LocalVariables|Get玩家編號)
        (:0
          (LocalVariables|Set是否是監聽伺服器的主人? (not (Networking|IsDedicatedServer))))
        (:1
          _))
      (Utilities|FlowControl|Sequence
        (:then_0
          ;[1 1 1] 生成玩家角色
          (switch Utilities|FlowControl|Switch|SwitchonE_Team (LocalVariables|Get玩家陣營)
            (:NewEnumerator1
              (bind _returnvalue_2 (Actor|GetActorOfClass "/Game/_Waraces/Blueprints/SpawnPoints/Player/Actor_Player_SpawnPoint_Red.Actor_Player_SpawnPoint_Red_C"))
              (LocalVariables|Set玩家出生點 (Transformation|GetActorTransform _returnvalue_2)))
            (:NewEnumerator2
              (bind _returnvalue_3 (Actor|GetActorOfClass "/Game/_Waraces/Blueprints/SpawnPoints/Player/Actor_Player_SpawnPoint_Blue.Actor_Player_SpawnPoint_Blue_C"))
              (LocalVariables|Set玩家出生點 (Transformation|GetActorTransform _returnvalue_3))))
          (bind _returnvalue_4 (Game|SpawnActorfromClass "/Game/_Waraces/Player/Blueprints/VRPawn_Main.VRPawn_Main_C" (LocalVariables|Get玩家出生點) "Undefined" 玩家控制器 (LocalVariables|Get玩家陣營) (LocalVariables|Get是否是監聽伺服器的主人?) (LocalVariables|Get玩家編號) 0))
          (Pawn|Possess 玩家控制器 _returnvalue_4))
        (:then_1
          ;[1 1 1] 把隊伍資料存進 PlayerState
          (bind _asps (Utilities|Casting|CastToPS (Variables|/Script/Engine.Controller|GetPlayerState 玩家控制器)))
          (Variables|/Game/_Waraces/Blueprints/GamePlay/PS.PS_C|Set所屬陣營 _asps (LocalVariables|Get玩家陣營)))
        (:then_2
          ;[1 1 1] 生成生命水晶
          (bind _水晶生成位置 (CallFunction|計算生命水晶的生成位置 (LocalVariables|Get玩家陣營) _returnvalue))
          (Game|SpawnActorfromClass "/Game/_Waraces/Blueprints/Crystal/BP_Crystal.BP_Crystal_C" _水晶生成位置 "AlwaysSpawn" 玩家控制器 _returnvalue (LocalVariables|Get玩家陣營) 0))))))

(fn 計算生命水晶的生成位置
  (params (水晶隸屬陣營 :type E_Team%20Enum :default "NewEnumerator0") (水晶編號 :type Integer))
  (switch Utilities|FlowControl|Switch|SwitchonE_Team 水晶隸屬陣營
    (:NewEnumerator1
      (switch int 水晶編號
        (:0
          (LocalVariables|Set水晶生成點 (Math|Transform|MakeTransform "605.000000,1250.000000,375.000000" "0, 0, 0" "2.000000,2.000000,2.000000")))
        (:1
          (LocalVariables|Set水晶生成點 (Math|Transform|MakeTransform "750.000000,1010.000000,375.000000" "0, 0, 0" "2.000000,2.000000,2.000000")))
        (:2
          (LocalVariables|Set水晶生成點 (Math|Transform|MakeTransform "895.000000,770.000000,375.000000" "0, 0, 0" "2.000000,2.000000,2.000000")))))
    (:NewEnumerator2
      (switch int 水晶編號
        (:0
          (LocalVariables|Set水晶生成點 (Math|Transform|MakeTransform "-615.000000,-1385.000000,375.000000" "0, 0, 0" "2.000000,2.000000,2.000000")))
        (:1
          (LocalVariables|Set水晶生成點 (Math|Transform|MakeTransform "-760.000000,-1145.000000,375.000000" "0, 0, 0" "2.000000,2.000000,2.000000")))
        (:2
          (LocalVariables|Set水晶生成點 (Math|Transform|MakeTransform "-905.000000,-905.000000,375.000000" "0, 0, 0" "2.000000,2.000000,2.000000"))))))
  (return (LocalVariables|Get水晶生成點)))

(fn 生成身份證
  (return (Guid|NewGuid)))

(fn 是否曾註冊在玩家名單中?
  (params (身份證 :type Guid%20Structure))
  (if (Guid|IsValidGuid 身份證)
    (bind _array_element (Utilities|Array|ForEachLoopwithBreak (Variables|Default|Get玩家名單) :!label _label)
      (:LoopBody
        (if (== 身份證 (.身份證 (Utilities|Struct|BreakStruct_PlayerList _array_element)))
          (LocalVariables|Set是否為回歸者? true)
          (goto _label Break)))
      (:Completed
        (return (LocalVariables|Get是否為回歸者?))))
    (else
      (return (LocalVariables|Get是否為回歸者?)))))

(fn 取得所有玩家的PS
  (for _array_element (Variables|Default|Get玩家名單)
    (bind _asps (Utilities|Casting|CastToPS (Variables|/Script/Engine.Controller|GetPlayerState (.玩家控制器 (Utilities|Struct|BreakStruct_PlayerList _array_element)))))
    (Utilities|Array|Add (LocalVariables|GetPS) _asps))
  (return (LocalVariables|GetPS)))

(fn 創建觀眾角色
  (params (玩家控制器 :type PC%20Object%20Reference))
  (bind _returnvalue (Actor|GetActorOfClass (.OutItem (Utilities|Array|Random (Utilities|Array|MakeArray "/Game/_Waraces/Blueprints/SpawnPoints/Player/Actor_Player_SpawnPoint_Red.Actor_Player_SpawnPoint_Red_C" "/Game/_Waraces/Blueprints/SpawnPoints/Player/Actor_Player_SpawnPoint_Blue.Actor_Player_SpawnPoint_Blue_C")))))
  (bind _returnvalue_2 (Game|SpawnActorfromClass "/Game/_Waraces/Player/Blueprints/SP.SP_C" (Transformation|GetActorTransform _returnvalue) "Undefined" 0 0))
  (Pawn|Possess 玩家控制器 _returnvalue_2))

(fn 隨機抽牌
  (params (卡牌種類 :type E_Card_Type%20Enum :default "NewEnumerator0") (要排除的效果 :type Array%20of%20E_Buff%20Enums :default "NewEnumerator4"))
  (switch Utilities|FlowControl|Switch|SwitchonE_Card_Type 卡牌種類
    (:NewEnumerator1
      (switch int (Math|Random|RandomInteger 3)
        (:0
          (bind _output_get (LocalVariables|Set卡牌資料表 "/Game/_Waraces/Cards/Character_Cards/Datas/DT_Character_Human.DT_Character_Human"))
          (bind _outrownames (DataTable|GetDataTableRowNames _output_get))
          (bind _returnvalue (Utilities|GetDataTableRow (LocalVariables|Get卡牌資料表) (.OutItem (Utilities|Array|Random _outrownames)))
            (:then
              (LocalVariables|Set角色種類%20 (.角色種類 (Utilities|Struct|BreakST_CharacterInfo_Human _returnvalue))))))
        (:1
          (bind _output_get_2 (LocalVariables|Set卡牌資料表 "/Game/_Waraces/Cards/Character_Cards/Datas/DT_Character_Beast.DT_Character_Beast"))
          (bind _outrownames_2 (DataTable|GetDataTableRowNames _output_get_2))
          (bind _returnvalue_2 (Utilities|GetDataTableRow (LocalVariables|Get卡牌資料表) (.OutItem (Utilities|Array|Random _outrownames_2)))
            (:then
              (LocalVariables|Set角色種類%20 (.角色種類 (Utilities|Struct|BreakST_CharacterInfo_Beast _returnvalue_2))))))
        (:2
          (bind _output_get_3 (LocalVariables|Set卡牌資料表 "/Game/_Waraces/Cards/Character_Cards/Datas/DT_Character_Goblin.DT_Character_Goblin"))
          (bind _outrownames_3 (DataTable|GetDataTableRowNames _output_get_3 :!label _label))
          (bind _returnvalue_3 (Utilities|GetDataTableRow (LocalVariables|Get卡牌資料表) (.OutItem (Utilities|Array|Random _outrownames_3)))
            (:then
              (if (Utilities|Enum|Equal(Enum) (.角色種類 (Utilities|Struct|BreakST_CharacterInfo_Goblin _returnvalue_3)) "NewEnumerator6")
                (goto _label)
                (else
                  (LocalVariables|Set角色種類%20 (.角色種類 (Utilities|Struct|BreakST_CharacterInfo_Goblin _returnvalue_3)))))))))
      (return (LocalVariables|Get角色種類%20) "NewEnumerator4" 卡牌種類))
    (:NewEnumerator2
      (bind _output_get_4 (LocalVariables|Set卡牌資料表 "/Game/_Waraces/Cards/Effect_Cards/Datas/DT_BuffCard.DT_BuffCard"))
      (bind _outrownames_4 (DataTable|GetDataTableRowNames _output_get_4 :!label _label_2))
      (bind _returnvalue_4 (Utilities|GetDataTableRow (LocalVariables|Get卡牌資料表) (.OutItem (Utilities|Array|Random _outrownames_4)))
        (:then
          (if (Utilities|Array|ContainsItem 要排除的效果 (.效果種類 (Utilities|Struct|BreakST_BuffCardInfo _returnvalue_4)))
            (goto _label_2)
            (else
              (return "NewEnumerator0" (.效果種類 (Utilities|Struct|BreakST_BuffCardInfo _returnvalue_4)) 卡牌種類))))))))