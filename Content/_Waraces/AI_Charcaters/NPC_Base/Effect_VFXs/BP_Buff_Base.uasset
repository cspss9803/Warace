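; BP_Buff_Base is a base Blueprint for NPC buff effects that finds pawns within an area.
; Its Trigger event calls SpawnBuff, which runs a single sphere overlap using a configurable radius, optionally ignoring the instigator.
; Each actor found is passed to the OnBuffOverlapActor dispatcher, so this graph handles only detection and applies no buff itself.
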(event Custom|Trigger
  (CallFunction|SpawnBuff))

(event Custom|SpawnBuff
  (bind _outactors (Collision|SphereOverlapActors "0, 0, 0" (Variables|Default|GetSphere%20Radius) (Utilities|Array|MakeArray "ObjectTypeQuery3") 0 (select (Variables|Default|GetIgnore%20Instigator) (Utilities|Array|MakeArray (Game|GetInstigator)) 0)))
  (for _array_element _outactors
    (Default|CallOnBuffOverlapActor _array_element)))

(fn ConstructionScript)