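; BP_NPC_HammerBeast is the hammer beast NPC, a child Blueprint that plugs its own attacks into inherited behavior.
; BeginPlay assigns the normal and advanced attack montages, the latter a looping attack, before calling the parent.
; WeaponTransform converts the static mesh's hand_l socket location into RightHand bone space with neutral rotation and scale, apparently for left-hand placement on the weapon.
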(event EventBeginPlay
  (Variables|Default|Set普通攻擊_Montage "/Game/_AI/NPC_HeavyHammer/動作/attack01_Montage.attack01_Montage")
  (Variables|Default|Set進階攻擊_Montage "/Game/_AI/NPC_HeavyHammer/動作/Anim_Attack01_Loop_Montage.Anim_Attack01_Loop_Montage")
  (|CallParentFunction))

(event Collision|EventActorBeginOverlap
  (params (OtherActor :type Actor%20Object%20Reference)))

(event EventTick
  (params (DeltaSeconds :type Float%20%28single-precision%29)))

(fn ConstructionScript
  (|CallParentFunction))

(fn WeaponTransform
  (bind _staticmesh (Variables|Default|GetStaticMesh))
  (Utilities|IsValid _staticmesh
    (:Is%20Valid
      (return (Math|Transform|MakeTransform (.OutPosition (Class|SkinnedMeshComponent|TransformtoBoneSpace (Variables|Character|GetMesh) "RightHand" (.location (Transformation|GetSocketTransform _staticmesh "hand_l" "RTS_World")) "0, 0, 0")) "0, 0, 0" "1.000000,1.000000,1.000000")))))