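; Tornado (龍捲風) variant of an over-time area-of-effect attack, filed under the AI attacks.
; It overrides Trigger to call the parent, which presumably handles the sustained damage, then adds the storm visuals and sound.
; The NS_ky_storm system attaches to the root component, while the tornado sound plays once triggered at the actor's location.
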(event EventBeginPlay
  (|CallParentFunction) ; This node is disabled and will not be called.\nDrag off pins to build functionality.
)

(event Collision|EventActorBeginOverlap
  (params (OtherActor :type Actor%20Object%20Reference))
  (|CallParentFunction OtherActor) ; This node is disabled and will not be called.\nDrag off pins to build functionality.
)

(event EventTick
  (params (DeltaSeconds :type Float%20%28single-precision%29))
  (|CallParentFunction DeltaSeconds) ; This node is disabled and will not be called.\nDrag off pins to build functionality.
)

(event EventTrigger
  (|CallParentFunction)
  (Niagara|SpawnSystemAttached "/Game/_AI/NPC_Goblin/特效/龍捲風/NS_ky_storm.NS_ky_storm" (Variables|Default|GetDefaultSceneRoot) "None" "0, 0, 0" "0, 0, 0" "KeepRelativeOffset" false)
  (Audio|PlaySoundatLocation "/Game/_AI/NPC_Goblin/音效/龍捲風音效.龍捲風音效" (Transformation|GetActorLocation self) "0, 0, 0" 1.0 1.0 0.0 0 0 0 0))

(fn ConstructionScript
  (|CallParentFunction))