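; An area-of-effect attack actor, named as an over-time ground crack, that adds crack visuals and impact audio to the hit behavior it inherits.
; Its HitActor override, commented as one-time damage, runs the parent logic, then calls a crack-summoning event on the root component.
; That event spawns an auto-destroying advanced-attack effect attached to the root and plays a hammer ground-hit sound at the actor's location.
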(event Custom|召喚地裂
  (params (AttachToComponent :type Scene%20Component%20Object%20Reference))
  (Niagara|SpawnSystemAttached (Variables|Default|Get進階攻擊特效) AttachToComponent "None" "0, 0, 0" "0, 0, 0" "KeepRelativeOffset" true)
  (Audio|PlaySoundatLocation "/Game/_AI/NPC_Stick/VFX/Crack/Crack_Orange/SFX/Sfx_Hit_Ground_Hammer_Cue.Sfx_Hit_Ground_Hammer_Cue" (Transformation|GetActorLocation self) "0, 0, 0" 1.0 1.0 0.0 0 0 0 0))

(event EventBeginPlay
  (|CallParentFunction) ; This node is disabled and will not be called.\nDrag off pins to build functionality.
)

(event Collision|EventActorBeginOverlap
  (params (OtherActor :type Actor%20Object%20Reference))
  (|CallParentFunction OtherActor) ; This node is disabled and will not be called.\nDrag off pins to build functionality.
)

(event EventTick
  (params (DeltaSeconds :type Float%20%28single-precision%29))
  (|CallParentFunction DeltaSeconds) ; This node is disabled and will not be called.\nDrag off pins to build functionality.
)

(event EventHitActor
  (|CallParentFunction)
  (CallFunction|召喚地裂 (Variables|Default|GetDefaultSceneRoot)))

(fn ConstructionScript
  (|CallParentFunction))