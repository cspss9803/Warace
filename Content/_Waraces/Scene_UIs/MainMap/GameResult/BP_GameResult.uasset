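; BP_GameResult is a world-space actor that shows the match result and plays a win or lose sound.
; On BeginPlay it creates WB_GameResult from the win flag (是否獲勝), assigns it to its widget component and shifts itself back, away from the camera.
; A gate then lets Tick rotate the widget to face the player camera each frame.
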(event EventBeginPlay
  (bind _returnvalue (Game|GetPlayerCameraManager 0))
  (bind _widget (Variables|Default|GetWidget))
  (bind _returnvalue_2 (Camera|GetCameraLocation _returnvalue))
  (bind _returnvalue_3 (Transformation|GetWorldLocation _widget))
  (bind _returnvalue_4 (Math|Rotator|FindLookatRotation _returnvalue_3 _returnvalue_2))
  (bind _returnvalue_5 (UserInterface|CreateWidget "/Game/_Waraces/Scene_UIs/MainMap/GameResult/WB_GameResult.WB_GameResult_C" 0 (Variables|Default|Get是否獲勝?)))
  (UserInterface|SetWidget (Variables|Default|GetWidget) _returnvalue_5)
  (Transformation|SetActorLocation (+ (Transformation|GetActorLocation) (* (Math|Vector|GetForwardVector _returnvalue_4) -1.5e+02)) false false)
  (Utilities|FlowControl|Sequence
    (:then_0
      (Variables|Default|GetWidget
        (:then
          (Utilities|FlowControl|Gate true) ; enters at Open
        )
        (:else)))
    (:then_1
      (Audio|PlaySound2D (select (Variables|Default|Get是否獲勝?) "/Game/_Waraces/Scene_UIs/MainMap/GameResult/SW_you_win.SW_you_win" "/Game/_Waraces/Scene_UIs/MainMap/GameResult/SW_you_lose.SW_you_lose") 1.0 1.0 0.0 0 0))))

(event EventTick
  (params (DeltaSeconds :type Float%20%28single-precision%29))
  (Utilities|FlowControl|Gate true
    (:Exit
      (bind _widget (Variables|Default|GetWidget)
        (:then
          (Transformation|SetWorldRotation _widget (Math|Rotator|FindLookatRotation (Transformation|GetWorldLocation (Variables|Default|GetWidget)) (Camera|GetCameraLocation (Game|GetPlayerCameraManager 0))) false false))
        (:else)))))

(fn ConstructionScript)