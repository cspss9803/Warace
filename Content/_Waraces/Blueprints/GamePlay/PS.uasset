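; PlayerState for a team battle game, holding each player's name, team, battle score and queue of battle characters.
; On BeginPlay it polls each tick until a team is set, caches that team's spawn point, and syncs the GameInstance name through client/server RPCs.
; A spawn event creates and dequeues the first queued character.
; RepNotifies refresh the 3D player list; nonzero scores also destroy remaining NPCs and advance the server's game phase.
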(event EventBeginPlay
  (Utilities|FlowControl|Sequence
    (:then_0
      (|儲存對戰角色的生成位置))
    (:then_1
      (|把GameInstance中儲存的玩家名稱儲存到PlayerState))))

(fn ConstructionScript)

(fn OnRepBattleScore
  (|是否要進行重置
    (:更新記分板就好
      (|更新記分板 :!label _label))
    (:重置
      (Utilities|FlowControl|Sequence
        (:then_0
          (goto _label))
        (:then_1
          (|清除戰鬥結束後還留在場上的所有對戰角色))
        (:then_2
          (|檢查是否滿足勝利條件))))))

(fn OnRepUserName
  (bind _returnvalue (Actor|GetActorOfClass "/Game/_Waraces/Scene_UIs/MainMap/PlayerList/Actor_3D_Widget_PlayerList.Actor_3D_Widget_PlayerList_C"))
  (Default|UpdatePlayerList _returnvalue))

(event Custom|setName_RunOnServer
  (params (UserName :type Text))
  (Variables|Default|SetUserName UserName))

(event Custom|GetPlayerName_RunOnOwningClient
  (bind _gi (CallFunction|取得遊戲實例))
  (bind _playername (Variables|/Game/_Waraces/Blueprints/GamePlay/GI.GI_C|GetPlayerName _gi))
  (Networking|SwitchHasAuthority
    (:Authority
      (Variables|Default|SetUserName _playername))
    (:Remote
      (CallFunction|SetNameRunonServer _playername) ; 轉為伺服器的身分去執行此事件
    )))

(event Custom|生成對戰角色
  (bind _對戰角色列表 (Variables|Default|Get對戰角色列表))
  (bind _output (Utilities|Array|Get(acopy) _對戰角色列表))
  (bind _charactertype (Utilities|Struct|BreakStruct_NPCData _output))
  (bind _returnvalue (Game|SpawnActorfromClass (CallFunction|取得NPC的Class _charactertype) (Variables|Default|GetBattleCharacterSpawnPotin) "AlwaysSpawn" (PlayerState|GetPawn) (Variables|Default|Get所屬陣營) _charactertype (Utilities|Array|MakeArray "NewEnumerator21" "NewEnumerator14") 0))
  (Variables|Default|Set目前的對戰角色 _returnvalue)
  (Utilities|Array|RemoveIndex (Variables|Default|Get對戰角色列表)))