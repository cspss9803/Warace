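; Small goblin NPC Blueprint that implements the creature's networked death sequence.
; Its death event switches the NPC AI controller to an empty behavior tree, calls a multicast event and disables capsule collision.
; The multicast plays the death montage, whose notify triggers the 播放死亡動畫 (play death animation) call on authority only, with both holy-wing protection and hell-summon effect flags off.
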(event Custom|小哥布林死亡
  (bind _asnpc_aicontroller (Utilities|Casting|CastToNPC_AIcontroller (Pawn|GetController)))
  (AI|RunBehaviorTree _asnpc_aicontroller "/Game/_AI/NPC_Blueprints/BehaviorTree/BT_Empty.BT_Empty")
  (CallFunction|小哥布林死亡Multicast)
  (Collision|SetCollisionEnabled (Variables|Default|GetCapsuleComponent) "NoCollision"))

(event Custom|小哥布林死亡Multicast
  (Animation|Montage|PlayMontage (Variables|Character|GetMesh) "/Game/_AI/NPC_S_Goblin/Animations/AM_sGoblin_Death.AM_sGoblin_Death"
    (:OnNotifyBegin
      (Networking|SwitchHasAuthority
        (:Authority
          (CallFunction|播放死亡動畫 false false))))))

(event EventBeginPlay
  (|CallParentFunction))

(fn ConstructionScript
  (|CallParentFunction))