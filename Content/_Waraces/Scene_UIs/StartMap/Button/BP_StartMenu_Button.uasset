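; Start menu 3D button actor for room create/join, IP connect, rename, tutorial and quit, using button and prompt widget components.
; On BeginPlay, ButtonType picks label and icon, links both widgets to the actor, or destroys it if None.
; An empty GameInstance PlayerName shrinks the button's draw size to hide it.
; Fade events animate every button instance, collapsing draw size after a delayed fade-out and restoring it on fade-in.
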(event Custom|ScaleFadeInAllButton
  (bind _outactors (Actor|GetAllActorsOfClass "BP_StartMenu_Button_C"))
  (for _array_element _outactors
    (Default|PlayScaleFadeOut (Variables|BP_StartMenu_Button_C|GetRef_BW_Button _array_element) "Reverse"))
  (bind _outactors_2 (Actor|GetAllActorsOfClass "BP_StartMenu_Button_C"))
  (for _array_element_2 _outactors_2
    (Class|WidgetComponent|SetDrawSize (Variables|BP_StartMenu_Button_C|GetWidgetComponent_Button _array_element_2) "(X=500.000000,Y=500.000000)")))

(event Custom|ScaleFadeOutAllButton
  (bind _outactors (Actor|GetAllActorsOfClass "BP_StartMenu_Button_C"))
  (for _array_element _outactors
    (Default|PlayScaleFadeOut (Variables|BP_StartMenu_Button_C|GetRef_BW_Button _array_element) "Forward"))
  (Utilities|FlowControl|Delay 1.0)
  (bind _outactors_2 (Actor|GetAllActorsOfClass "BP_StartMenu_Button_C"))
  (for _array_element_2 _outactors_2
    (Class|WidgetComponent|SetDrawSize (Variables|BP_StartMenu_Button_C|GetWidgetComponent_Button _array_element_2) "(X=1.000000,Y=1.000000)")))

(event EventBeginPlay
  (bind _widgetcomponent_button (Variables|Default|GetWidgetComponent_Button))
  (bind _aswb_button_prompt (Utilities|Casting|CastToWB_ButtonPrompt (UserInterface|GetWidget (Variables|Default|GetWidgetComponent_ButtonPrompt))))
  (switch Utilities|FlowControl|Switch|SwitchonE_ButtonType (Variables|ButtonSetting|GetButtonType)
    (:NewEnumerator3
      (Actor|DestroyActor))
    (:NewEnumerator0
      (Variables|Default|SetButtonPromptText "創建房間")
      (Variables|Default|SetButtonIcon "/Game/_Waraces/Scene_UIs/StartMap/Button/Textures/T_CreateRoom.T_CreateRoom")
      (Variables|/Game/_Waraces/Scene_UIs/StartMap/Button/WB_ButtonPrompt.WB_ButtonPrompt_C|SetButtonPromptText _aswb_button_prompt (Variables|Default|GetButtonPromptText) :!label _label)
      (bind _aswb_button (Utilities|Casting|CastToWB_Button (UserInterface|GetWidget (Variables|Default|GetWidgetComponent_Button))))
      (bind _output_get (Variables|Default|SetRef_BW_Button _aswb_button))
      (Variables|/Game/_Waraces/Scene_UIs/StartMap/Button/WB_Button.WB_Button_C|SetRef_BW_ButtonPrompt _output_get _aswb_button_prompt)
      (Variables|/Game/_Waraces/Scene_UIs/StartMap/Button/WB_Button.WB_Button_C|SetButtonType (Variables|Default|GetRef_BW_Button) (Variables|ButtonSetting|GetButtonType))
      (Class|Image|SetBrush (Variables|/Game/_Waraces/Scene_UIs/StartMap/Button/WB_Button.WB_Button_C|Geticon (Variables|Default|GetRef_BW_Button)) (Utilities|Struct|MakeSlateBrush "Image" "NoTile" "NoMirror" "(X=250.000000,Y=250.000000)" "(Left=0.000000,Top=0.000000,Right=0.000000,Bottom=0.000000)" "(SpecifiedColor=(R=1.000000,G=1.000000,B=1.000000,A=1.000000),ColorUseRule=UseColor_Specified)" "(CornerRadii=(X=0.000000,Y=0.000000,Z=0.000000,W=1.000000),Color=(SpecifiedColor=(R=0.000000,G=0.000000,B=0.000000,A=0.000000),ColorUseRule=UseColor_Specified),Width=0.000000,RoundingType=HalfHeightRadius,bUseBrushTransparency=False)" (Variables|Default|GetButtonIcon)))
      (Variables|/Game/_Waraces/Scene_UIs/StartMap/Button/WB_Button.WB_Button_C|SetRef_Actor_3D_Widget_Button (Variables|Default|GetRef_BW_Button) self)
      (bind _asgi (Utilities|Casting|CastToGI (Game|GetGameInstance)))
      (if (Utilities|Text|TextIsEmpty (Variables|/Game/_Waraces/Blueprints/GamePlay/GI.GI_C|GetPlayerName _asgi))
        (bind _asgi_2 (Utilities|Casting|CastToGI (Game|GetGameInstance)))
        (if (Utilities|Text|TextIsEmpty (Variables|/Game/_Waraces/Blueprints/GamePlay/GI.GI_C|GetPlayerName _asgi_2))
          (Class|WidgetComponent|SetDrawSize _widgetcomponent_button "(X=1.000000,Y=1.000000)")
          (else
            (Class|WidgetComponent|SetDrawSize _widgetcomponent_button "(X=500.000000,Y=500.000000)")
            (Widget|SetVisibility (Variables|/Game/_Waraces/Scene_UIs/StartMap/Button/WB_Button.WB_Button_C|GetButton (Variables|Default|GetRef_BW_Button)) "Visible")))))
    (:NewEnumerator1
      (Variables|Default|SetButtonPromptText "開始連線")
      (Variables|Default|SetButtonIcon "/Game/_Waraces/Scene_UIs/StartMap/Button/Textures/T_ConnectRoom.T_ConnectRoom")
      (goto _label))
    (:NewEnumerator4
      (Variables|Default|SetButtonPromptText "重新命名")
      (Variables|Default|SetButtonIcon "/Game/_Waraces/Scene_UIs/StartMap/Button/Textures/T_Rename.T_Rename")
      (goto _label))
    (:NewEnumerator2
      (Variables|Default|SetButtonPromptText "離開遊戲")
      (Variables|Default|SetButtonIcon "/Game/_Waraces/Scene_UIs/StartMap/Button/Textures/T_QuitGame.T_QuitGame")
      (goto _label))
    (:NewEnumerator5
      (Variables|Default|SetButtonPromptText "IP連線")
      (Variables|Default|SetButtonIcon "/Game/_Waraces/Scene_UIs/StartMap/Button/Textures/T_IP_Connect.T_IP_Connect")
      (goto _label))
    (:NewEnumerator6
      (Variables|Default|SetButtonPromptText "新手導覽")
      (Variables|Default|SetButtonIcon "/Game/_Waraces/Scene_UIs/StartMap/Button/Textures/T_Guide.T_Guide")
      (goto _label))))

(fn ConstructionScript)