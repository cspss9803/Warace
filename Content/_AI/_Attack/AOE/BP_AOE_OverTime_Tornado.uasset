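; Tornado variant of an over-time AOE attack, adding the visual and sound for a damage-over-time effect.
; On Trigger it runs the parent logic, then calls 召喚龍捲風 (summon tornado) on its root component.
; That event spawns the NS_ky_storm particle system attached to the given component and plays the tornado sound at the actor's location.
; No damage logic lives in this Blueprint itself.
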(event Custom|召喚龍捲風
  (params (AttachToComponent :type Scene%20Component%20Object%20Reference))
  (Niagara|SpawnSystemAttached "/Game/_AI/NPC_Goblin/VFX/tornado/NS_ky_storm.NS_ky_storm" AttachToComponent "None" "0, 0, 0" "0, 0, 0" "KeepRelativeOffset" false)
  (Audio|PlaySoundatLocation "/Game/_AI/NPC_Goblin/Audio/龍捲風音效.龍捲風音效" (Transformation|GetActorLocation self) "0, 0, 0" 1.0 1.0 0.0 0 0 0 0))

(event EventBeginPlay
  (|CallParentFunction) ; This node is disabled and will not be called.\nDrag off pins to build functionality.
)

(event Collision|EventActorBeginOverlap
  (params (OtherActor :type Actor%20Object%20Reference))
  (|CallParentFunction OtherActor) ; This node is disabled and will not be called.\nDrag off pins to build functionality.
)

(event EventTick
  (params (DeltaSeconds :type Float%20%28single-precision%29))
  (|CallParentFunction DeltaSeconds) ; This node is disabled and will not be called.\nDrag off pins to build functionality.
)

(event EventTrigger
  (|CallParentFunction)
  (CallFunction|召喚龍捲風 (Variables|Default|GetDefaultSceneRoot)))

(fn ConstructionScript
  (|CallParentFunction))