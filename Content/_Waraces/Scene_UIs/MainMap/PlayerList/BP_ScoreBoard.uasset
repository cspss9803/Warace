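; Scoreboard actor that shows the name and battle score of one Red team and one Blue team player through a WB_ScoreBoard widget component.
; BeginPlay caches the widget's text elements.
; UpdatePlayerList finds team PlayerStates in the GameState's PlayerArray, then refreshes each valid side.
; Name updates retry next tick until widget and username are ready, with a debug flag to show PlayerId instead.
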(event Custom|UpdatePlayerList
  (if (|是否雙方陣營的PlayerState都被存起來了?)
    _
    (else
      (|將雙方陣營的PlayerState存起來
        (:OutputPin
          _))))
  (Utilities|FlowControl|Sequence
    (:then_0
      (Utilities|IsValid (Variables|Default|GetPlayerState_Red) ; 紅隊的 PlayerState 是否準備好了?
        (:Is%20Valid
          (|更新紅隊資料))))
    (:then_1
      (Utilities|IsValid (Variables|Default|GetPlayerState_Blue) ; 藍隊的 PlayerState 是否準備好了?
        (:Is%20Valid
          (|更新藍隊資料))))))

(event EventBeginPlay
  (bind _aswb_score_board (Utilities|Casting|CastToWB_ScoreBoard (UserInterface|GetWidget (Variables|Default|GetWidgetComponent_PlayerList))))
  (Variables|Default|SetPlayer%20Name%20Red (Variables|/Game/_Waraces/Scene_UIs/MainMap/PlayerList/WB_ScoreBoard.WB_ScoreBoard_C|GetPlayerName_Red _aswb_score_board)) ; 紅隊玩家名稱的 Widget 元件
  (Variables|Default|SetPlayer%20Name%20Blue (Variables|/Game/_Waraces/Scene_UIs/MainMap/PlayerList/WB_ScoreBoard.WB_ScoreBoard_C|GetPlayerName_Blue _aswb_score_board)) ; 藍隊玩家名稱的 Widget 元件
  (Variables|Default|SetScore%20Red (Variables|/Game/_Waraces/Scene_UIs/MainMap/PlayerList/WB_ScoreBoard.WB_ScoreBoard_C|GetScore_Red _aswb_score_board)) ; 紅隊玩家分數的 Widget 元件
  (Variables|Default|SetScore%20Blue (Variables|/Game/_Waraces/Scene_UIs/MainMap/PlayerList/WB_ScoreBoard.WB_ScoreBoard_C|GetScore_Blue _aswb_score_board)) ; 藍隊玩家分數的 Widget 元件
)

(fn ConstructionScript)