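; BP_Buff_復活 is a short-lived card VFX actor that plays a revive (復活) effect aimed at the revived character's position.
; On BeginPlay it tints its Niagara component red or green for one of two accepted effect enum values and passes it the target location.
; It zeroes the projectile count after a second, then destroys itself three seconds later.
; Any other effect value prints an error and destroys the actor immediately.
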(event EventBeginPlay
  (bind _效果 (Variables|Default|Get效果))
  (bind _niagara (Variables|Default|GetNiagara))
  (if (Utilities|Enum|Equal(Enum) _效果 "NewEnumerator6")
    (Effects|Components|ParticleSystem|SetColorParameter (Variables|Default|GetNiagara) "Color" "(R=0.679543,G=0.049707,B=0.035601,A=1.000000)")
    (Effects|Components|ParticleSystem|SetVectorParameter _niagara "TargetLoaction" (Variables|Default|Get復活者位置) :!label _label)
    (Utilities|FlowControl|Delay 1.0)
    (Effects|Components|ParticleSystem|SetFloatParameter _niagara "NumberOfProjectiles" 0.0)
    (Utilities|FlowControl|Delay 3.0)
    (Actor|DestroyActor)
    (elif (Utilities|Enum|Equal(Enum) _效果 "NewEnumerator19")
      (Effects|Components|ParticleSystem|SetColorParameter (Variables|Default|GetNiagara) "Color" "(R=0.282819,G=0.593750,B=0.280755,A=1.000000)")
      (goto _label)
      (else
        (Development|PrintString "BP_Buff_復活: 錯誤!  傳入的效果，並非復活效果" true true "(R=1.000000,G=0.043946,B=0.000000,A=1.000000)" 1e+02)
        (Actor|DestroyActor)))))

(fn ConstructionScript)