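; Shared Blueprint function library for a team-based card battle game, providing game framework accessors, NPC lookups and card helpers.
; NPC type maps to class, montages, color and race, with race selecting the DataTable for stats and card info.
; Slot helpers build five team-mirrored spawn transforms from a placed actor and find empty slots.
; Net-role macros distinguish dedicated server, listen host and owning client to report whether logic runs locally for a player.
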(fn 取得遊戲狀態
  (bind _asgs (Utilities|Casting|CastToGS (Game|GetGameState (LocalVariables|Get__WorldContext))))
  (return _asgs))

(fn 取得遊戲模式
  (bind _asgm (Utilities|Casting|CastToGM (Game|GetGameMode (LocalVariables|Get__WorldContext))))
  (return _asgm))

(fn 取得遊戲實例
  (bind _asgi (Utilities|Casting|CastToGI (Game|GetGameInstance (LocalVariables|Get__WorldContext))))
  (return _asgi))

(fn 取得NPC的Class
  (params (NPC%20的種類 :type E_NPC%20Enum :default "NewEnumerator0"))
  (switch Utilities|FlowControl|Switch|SwitchonE_NPC NPC%20的種類
    (:NewEnumerator0
      (return 0))
    (:NewEnumerator4
      (return "/Game/_Waraces/AI_Charcaters/NPC_Base/BP_NPC_Lava.BP_NPC_Lava_C"))
    (:NewEnumerator6
      (return "/Game/_Waraces/AI_Charcaters/NPC_Base/BP_S_Goblin.BP_S_Goblin_C"))
    (:NewEnumerator8
      (return "/Game/_Waraces/AI_Charcaters/NPC_Base/BP_NPC_Goblin.BP_NPC_Goblin_C"))
    (:NewEnumerator9
      (return "/Game/_Waraces/AI_Charcaters/NPC_Base/BP_NPC_Forest.BP_NPC_Forest_C"))
    (:NewEnumerator10
      (return "/Game/_Waraces/AI_Charcaters/NPC_Base/BP_NPC_Beast.BP_NPC_Beast_C"))
    (:NewEnumerator11
      (return "/Game/_Waraces/AI_Charcaters/NPC_Base/BP_NPC_SpearMan.BP_NPC_SpearMan_C"))
    (:NewEnumerator12
      (return "/Game/_Waraces/AI_Charcaters/NPC_Base/BP_NPC_Human.BP_NPC_Human_C"))
    (:NewEnumerator13
      (return "/Game/_Waraces/AI_Charcaters/NPC_Base/BP_NPC_Assassins.BP_NPC_Assassins_C"))
    (:NewEnumerator14
      (return "/Game/_Waraces/AI_Charcaters/NPC_Base/BP_NPC_Wolf.BP_NPC_Wolf_C"))
    (:NewEnumerator16
      (return "/Game/_Waraces/AI_Charcaters/NPC_Base/BP_NPC_Mallet.BP_NPC_Mallet_C"))))

(fn 取得NPC的蒙太奇攻擊動畫
  (params (NPC :type E_NPC%20Enum :default "NewEnumerator0"))
  (switch Utilities|FlowControl|Switch|SwitchonE_NPC NPC
    (:NewEnumerator0
      (return 0 0 0))
    (:NewEnumerator4
      (return "/Game/_Waraces/AI_Charcaters/NPC_Lava/Animations/AM_Lava_Attack_Normal.AM_Lava_Attack_Normal" "/Game/_Waraces/AI_Charcaters/NPC_Lava/Animations/AM_Lava_Attack_Advance.AM_Lava_Attack_Advance" "/Game/_Waraces/AI_Charcaters/NPC_Lava/Animations/AM_Lava_Death.AM_Lava_Death"))
    (:NewEnumerator6
      (return "/Game/_Waraces/AI_Charcaters/NPC_S_Goblin/Animations/AM_S_Goblin_Attack_Normal.AM_S_Goblin_Attack_Normal" "/Game/_Waraces/AI_Charcaters/NPC_S_Goblin/Animations/AM_S_Goblin_Attack_Normal.AM_S_Goblin_Attack_Normal" "/Game/_Waraces/AI_Charcaters/NPC_S_Goblin/Animations/AM_S_Goblin_Death.AM_S_Goblin_Death"))
    (:NewEnumerator8
      (return "/Game/_Waraces/AI_Charcaters/NPC_Goblin/Animations/AM_Goblin_Attack_Normal.AM_Goblin_Attack_Normal" "/Game/_Waraces/AI_Charcaters/NPC_Goblin/Animations/AM_Goblin_Attack_Advance.AM_Goblin_Attack_Advance" "/Game/_Waraces/AI_Charcaters/NPC_Goblin/Animations/AM_Goblin_Death.AM_Goblin_Death"))
    (:NewEnumerator9
      (return "/Game/_Waraces/AI_Charcaters/NPC_Forest/Animations/AM_Forest_Attack_Normal.AM_Forest_Attack_Normal" "/Game/_Waraces/AI_Charcaters/NPC_Forest/Animations/AM_Forest_Attack_Advance1.AM_Forest_Attack_Advance1" "/Game/_Waraces/AI_Charcaters/NPC_Forest/Animations/AM_Forest_Death.AM_Forest_Death"))
    (:NewEnumerator10
      (return "/Game/_Waraces/AI_Charcaters/NPC_Beast/Animations/AM_Beast_Attact_Normal.AM_Beast_Attact_Normal" "/Game/_Waraces/AI_Charcaters/NPC_Beast/Animations/AM_Beast_Attack_Advance.AM_Beast_Attack_Advance" "/Game/_Waraces/AI_Charcaters/NPC_Beast/Animations/AM_Beast_Death.AM_Beast_Death"))
    (:NewEnumerator11
      (return "/Game/_Waraces/AI_Charcaters/NPC_SpearMan/Animations/AM_SpearMan_Attack_Normal.AM_SpearMan_Attack_Normal" "/Game/_Waraces/AI_Charcaters/NPC_SpearMan/Animations/AM_SpearMan_Attack_Advance.AM_SpearMan_Attack_Advance" "/Game/_Waraces/AI_Charcaters/NPC_SpearMan/Animations/AM_SpearMan_Death.AM_SpearMan_Death"))
    (:NewEnumerator12
      (return "/Game/_Waraces/AI_Charcaters/NPC_Human/Animations/AM_Human_Attack_Normal.AM_Human_Attack_Normal" "/Game/_Waraces/AI_Charcaters/NPC_Human/Animations/AM_Human_Attack_Advance.AM_Human_Attack_Advance" "/Game/_Waraces/AI_Charcaters/NPC_Human/Animations/AM_Human_Death.AM_Human_Death"))
    (:NewEnumerator13
      (return "/Game/_Waraces/AI_Charcaters/NPC_Assassin/Animations/AM_Assassin_Attack_Normal.AM_Assassin_Attack_Normal" "/Game/_Waraces/AI_Charcaters/NPC_Assassin/Animations/AM_Assassin_Attack_Advance.AM_Assassin_Attack_Advance" "/Game/_Waraces/AI_Charcaters/NPC_Assassin/Animations/AM_Assassin_Death.AM_Assassin_Death"))
    (:NewEnumerator14
      (return "/Game/_Waraces/AI_Charcaters/NPC_Wolfman/Animations/AM_Wolf_Attack_Normal.AM_Wolf_Attack_Normal" "/Game/_Waraces/AI_Charcaters/NPC_Wolfman/Animations/AM_Wolf_Attack_Advance.AM_Wolf_Attack_Advance" "/Game/_Waraces/AI_Charcaters/NPC_Wolfman/Animations/AM_Wolf_Death.AM_Wolf_Death"))
    (:NewEnumerator16
      (return "/Game/_Waraces/AI_Charcaters/NPC_S_Goblin/Animations/AM_S_Goblin_Attack_Normal.AM_S_Goblin_Attack_Normal" "/Game/_Waraces/AI_Charcaters/NPC_S_Goblin/Animations/AM_S_Goblin_Attack_Normal.AM_S_Goblin_Attack_Normal" "/Game/_Waraces/AI_Charcaters/NPC_S_Goblin/Animations/AM_S_Goblin_Death.AM_S_Goblin_Death"))))

(fn 取得NPC的顏色
  (params (NPC :type E_NPC%20Enum :default "NewEnumerator0"))
  (switch Utilities|FlowControl|Switch|SwitchonE_NPC NPC
    (:NewEnumerator0
      (return "(R=0.000000,G=0.000000,B=0.000000,A=1.000000)"))
    (:NewEnumerator4
      (return "(R=1.000000,G=0.000000,B=0.000000,A=1.000000)"))
    (:NewEnumerator6
      (return "(R=0.336107,G=1.000000,B=0.000000,A=1.000000)"))
    (:NewEnumerator8
      (return "(R=0.000000,G=1.000000,B=0.043410,A=1.000000)"))
    (:NewEnumerator9
      (return "(R=0.933073,G=0.000000,B=1.000000,A=1.000000)"))
    (:NewEnumerator10
      (return "(R=0.040046,G=0.000000,B=1.000000,A=1.000000)"))
    (:NewEnumerator11
      (return "(R=1.000000,G=0.864395,B=0.000000,A=1.000000)"))
    (:NewEnumerator12
      (return "(R=1.000000,G=1.000000,B=1.000000,A=1.000000)"))
    (:NewEnumerator13
      (return "(R=0.000000,G=0.172219,B=1.000000,A=1.000000)"))
    (:NewEnumerator14
      (return "(R=1.000000,G=0.000000,B=0.036709,A=1.000000)"))
    (:NewEnumerator16
      (return "(R=1.000000,G=0.604977,B=0.169630,A=1.000000)"))))

(fn 取得NPC的種族
  (params (角色種類 :type E_NPC%20Enum :default "NewEnumerator0"))
  (switch Utilities|FlowControl|Switch|SwitchonE_NPC 角色種類
    (:NewEnumerator0
      (Development|PrintString 0 "錯誤: 取得NPC種族時發生錯誤，NPC是None" true true "(R=1.000000,G=0.000000,B=0.014578,A=1.000000)" 1e+03)
      (return "NewEnumerator0"))
    (:NewEnumerator4
      (return "NewEnumerator2"))
    (:NewEnumerator6
      (return "NewEnumerator2"))
    (:NewEnumerator8
      (return "NewEnumerator2"))
    (:NewEnumerator9
      (return "NewEnumerator2"))
    (:NewEnumerator10
      (return "NewEnumerator3"))
    (:NewEnumerator11
      (return "NewEnumerator1"))
    (:NewEnumerator12
      (return "NewEnumerator1"))
    (:NewEnumerator13
      (return "NewEnumerator1"))
    (:NewEnumerator14
      (return "NewEnumerator3"))
    (:NewEnumerator16
      (return "NewEnumerator3"))))

(fn 取得種族的圖示
  (params (種族 :type E_Races%20Enum :default "NewEnumerator0"))
  (switch Utilities|FlowControl|Switch|SwitchonE_Races 種族
    (:NewEnumerator0
      (return "/Game/_Waraces/Cards/Card_UIs/Card/T_CardIcon_None.T_CardIcon_None"))
    (:NewEnumerator1
      (return "/Game/_Waraces/Cards/Card_UIs/Card/T_CardIcon_Human.T_CardIcon_Human"))
    (:NewEnumerator3
      (return "/Game/_Waraces/Cards/Card_UIs/Card/T_CardIcon_Beast.T_CardIcon_Beast"))
    (:NewEnumerator2
      (return "/Game/_Waraces/Cards/Card_UIs/Card/T_CardIcon_Goblin.T_CardIcon_Goblin"))))

(fn 取得角色牌槽位的Class
  (params (陣營 :type E_Team%20Enum :default "NewEnumerator0"))
  (switch Utilities|FlowControl|Switch|SwitchonE_Team 陣營
    (:NewEnumerator0
      (return 0))
    (:NewEnumerator1
      (return "/Game/_Waraces/Blueprints/SpawnPoints/CardSlot/Actor_CardSlot0_SpawnPoint_Red.Actor_CardSlot0_SpawnPoint_Red_C"))
    (:NewEnumerator2
      (return "/Game/_Waraces/Blueprints/SpawnPoints/CardSlot/Actor_CardSlot0_SpawnPoint_Blue.Actor_CardSlot0_SpawnPoint_Blue_C"))))

(fn 取得角色槽位的生成位置
  (params (陣營 :type E_Team%20Enum :default "NewEnumerator0"))
  (bind _returnvalue (Actor|GetActorOfClass 0 (CallFunction|取得角色牌槽位的Class 陣營)))
  (LocalVariables|Set角色槽位的生成基點 (Transformation|GetActorTransform _returnvalue))
  (switch Utilities|FlowControl|Switch|SwitchonE_Team 陣營
    (:NewEnumerator1
      (LocalVariables|Set槽位間距 (* (LocalVariables|Get槽位間距) -1)))
    (:NewEnumerator2
      (LocalVariables|Set槽位間距 (* (LocalVariables|Get槽位間距) 1))))
  (for _index (range 0 4)
    (LocalVariables|SetIndex _index)
    (Utilities|Array|Add (LocalVariables|Get槽位生成位置) (Math|Transform|MakeTransform (Math|Vector|MakeVector (.x (.location (LocalVariables|Get角色槽位的生成基點))) (+ (* (LocalVariables|GetIndex) (LocalVariables|Get槽位間距)) (.y (.location (LocalVariables|Get角色槽位的生成基點)))) (.z (.location (LocalVariables|Get角色槽位的生成基點)))) (.rotation (LocalVariables|Get角色槽位的生成基點)) (.scale (LocalVariables|Get角色槽位的生成基點)))))
  (return (LocalVariables|Get槽位生成位置)))

(fn 取得敵方的陣營
  (params (我方陣營 :type E_Team%20Enum :default "NewEnumerator0"))
  (switch Utilities|FlowControl|Switch|SwitchonE_Team 我方陣營
    (:NewEnumerator1
      (return "NewEnumerator2"))
    (:NewEnumerator2
      (return "NewEnumerator1"))))

(fn 取得角色卡牌資訊
  (params (角色種類 :type E_NPC%20Enum :default "NewEnumerator0"))
  (bind _returnvalue (Utilities|String|EnumtoString 角色種類))
  (bind _returnvalue_2 (Utilities|String|StringToName _returnvalue))
  (switch Utilities|FlowControl|Switch|SwitchonE_Races (CallFunction|取得NPC的種族 角色種類 (LocalVariables|Get__WorldContext))
    (:NewEnumerator1
      (bind _returnvalue_3 (Utilities|GetDataTableRow "/Game/_Waraces/Cards/Character_Cards/Datas/DT_Character_Human.DT_Character_Human" _returnvalue_2)
        (:then
          (return (Utilities|Struct|MakeST_CharacterInfo_All (.角色種類 _returnvalue_3) (.角色名稱 _returnvalue_3) (.角色描述 _returnvalue_3) (.圖片 _returnvalue_3) (.攻擊力 _returnvalue_3) (.攻擊速度 _returnvalue_3) (.生命值 _returnvalue_3) (.魔力上限 _returnvalue_3) (.普攻回魔量 _returnvalue_3) (.進階攻擊所需魔量 _returnvalue_3) (.種族傷害倍率 _returnvalue_3) (.進階攻擊呼叫次數 _returnvalue_3))))))
    (:NewEnumerator3
      (bind _returnvalue_4 (Utilities|GetDataTableRow "/Game/_Waraces/Cards/Character_Cards/Datas/DT_Character_Beast.DT_Character_Beast" _returnvalue_2)
        (:then
          (return (Utilities|Struct|MakeST_CharacterInfo_All (.角色種類 _returnvalue_4) (.角色名稱 _returnvalue_4) (.角色描述 _returnvalue_4) (.圖片 _returnvalue_4) (.攻擊力 _returnvalue_4) (.攻擊速度 _returnvalue_4) (.生命值 _returnvalue_4) (.魔力上限 _returnvalue_4) (.普攻回魔量 _returnvalue_4) (.進階攻擊所需魔量 _returnvalue_4) (.種族傷害倍率 _returnvalue_4) (.進階攻擊呼叫次數 _returnvalue_4))))))
    (:NewEnumerator2
      (bind _returnvalue_5 (Utilities|GetDataTableRow "/Game/_Waraces/Cards/Character_Cards/Datas/DT_Character_Goblin.DT_Character_Goblin" _returnvalue_2)
        (:then
          (return (Utilities|Struct|MakeST_CharacterInfo_All (.角色種類 _returnvalue_5) (.角色名稱 _returnvalue_5) (.角色描述 _returnvalue_5) (.圖片 _returnvalue_5) (.攻擊力 _returnvalue_5) (.攻擊速度 _returnvalue_5) (.生命值 _returnvalue_5) (.魔力上限 _returnvalue_5) (.普攻回魔量 _returnvalue_5) (.進階攻擊所需魔量 _returnvalue_5) (.種族傷害倍率 _returnvalue_5) (.進階攻擊呼叫次數 _returnvalue_5))))))))

(fn 取得效果卡牌資訊
  (params (效果種類 :type E_Buff%20Enum :default "NewEnumerator4"))
  (bind _returnvalue (Utilities|GetDataTableRow "/Game/_Waraces/Cards/Effect_Cards/Datas/DT_BuffCard.DT_BuffCard" (Utilities|String|StringToName (Utilities|String|EnumtoString 效果種類)))
    (:then
      (return _returnvalue))))

(fn 隨機打亂卡牌順序
  (params (要打亂的卡牌們 :type Array%20of%20Widget%20Object%20References))
  (bind _output_get (LocalVariables|Set待打亂的卡牌們 要打亂的卡牌們))
  (Utilities|Array|Shuffle _output_get)
  (for _array_element (LocalVariables|Get待打亂的卡牌們)
    (bind _aswb_card (Utilities|Casting|CastToWB_Card _array_element))
    (Utilities|Array|Add (LocalVariables|Get已經打亂的卡牌們) _aswb_card))
  (return (LocalVariables|Get已經打亂的卡牌們)))

(fn 取得空的角色槽位
  (params (我方角色槽位 :type Array%20of%20BP%20Card%20Slot%20Object%20References) (玩家狀態 :type PS%20Object%20Reference))
  (for (_array_element _array_index) (Variables|/Game/_Waraces/Blueprints/GamePlay/PS.PS_C|Get對戰角色列表 玩家狀態)
    (if (Utilities|Enum|Equal(Enum) (.CharacterType (Utilities|Struct|BreakStruct_NPCData _array_element)) "NewEnumerator0")
      (Utilities|Array|Add (LocalVariables|Get空槽位的序號) _array_index)))
  (for _array_element_2 (LocalVariables|Get空槽位的序號)
    (Utilities|Array|Add (LocalVariables|Get空的角色槽位) (Utilities|Array|Get(acopy) 我方角色槽位 _array_element_2)))
  (return (LocalVariables|Get空的角色槽位)))

(fn 取得槽位上角色的種族
  (params (角色槽位 :type BP%20Card%20Slot%20Object%20Reference))
  (bind _目前生成在槽位上的展示角色 (Variables|/Game/_Waraces/Cards/Card_UIs/CardSlot/BP_CardSlot.BP_CardSlot_C|Get目前生成在槽位上的展示角色 角色槽位)
    (:then
      (bind _asbp_npc_display (Utilities|Casting|CastToBP_NPC_Display _目前生成在槽位上的展示角色)
        (:then
          (return (CallFunction|取得NPC的種族 (Variables|/Game/_Waraces/AI_Charcaters/NPC_Base/BP_NPC_Display.BP_NPC_Display_C|GetNPC%20種類 _asbp_npc_display) (LocalVariables|Get__WorldContext))))
        (:CastFailed
          (return "NewEnumerator0"))))
    (:else
      (return "NewEnumerator0"))))

(fn 此邏輯是否執行於該玩家的本地端上?
  (params (玩家角色 :type Pawn%20Object%20Reference))
  (|在哪個端上?
    (:伺服端
      (|是哪一種伺服端?
        (:獨立伺服器
          _)
        (:監聽伺服器
          (|是否伺服端主人的本地端
            (:是
              (return true))
            (:否
              _)))))
    (:用戶端
      (|在哪一種用戶端上?
        (:在自己的用戶端上
          (return true))
        (:在其他玩家的用戶端上
          _))))
  (return false))

(fn 取得角色屬性
  (params (角色種類 :type E_NPC%20Enum :default "NewEnumerator0"))
  (bind _returnvalue (Utilities|String|EnumtoString 角色種類))
  (bind _returnvalue_2 (Utilities|String|StringToName _returnvalue))
  (switch Utilities|FlowControl|Switch|SwitchonE_Races (CallFunction|取得NPC的種族 角色種類 (LocalVariables|Get__WorldContext))
    (:NewEnumerator1
      (bind _returnvalue_3 (Utilities|GetDataTableRow "/Game/_Waraces/Cards/Character_Cards/Datas/DT_Character_Human.DT_Character_Human" _returnvalue_2)
        (:then
          (return (.攻擊力 (Utilities|Struct|BreakST_CharacterInfo_Human _returnvalue_3)) (.攻擊速度 (Utilities|Struct|BreakST_CharacterInfo_Human _returnvalue_3)) (.生命值 (Utilities|Struct|BreakST_CharacterInfo_Human _returnvalue_3)) (.普攻回魔量 (Utilities|Struct|BreakST_CharacterInfo_Human _returnvalue_3)) (.進階攻擊所需魔量 (Utilities|Struct|BreakST_CharacterInfo_Human _returnvalue_3)) (.種族傷害倍率 (Utilities|Struct|BreakST_CharacterInfo_Human _returnvalue_3)) (.進階攻擊呼叫次數 (Utilities|Struct|BreakST_CharacterInfo_Human _returnvalue_3))))))
    (:NewEnumerator3
      (bind _returnvalue_4 (Utilities|GetDataTableRow "/Game/_Waraces/Cards/Character_Cards/Datas/DT_Character_Beast.DT_Character_Beast" _returnvalue_2)
        (:then
          (return (.攻擊力 (Utilities|Struct|BreakST_CharacterInfo_Beast _returnvalue_4)) (.攻擊速度 (Utilities|Struct|BreakST_CharacterInfo_Beast _returnvalue_4)) (.生命值 (Utilities|Struct|BreakST_CharacterInfo_Beast _returnvalue_4)) (.普攻回魔量 (Utilities|Struct|BreakST_CharacterInfo_Beast _returnvalue_4)) (.進階攻擊所需魔量 (Utilities|Struct|BreakST_CharacterInfo_Beast _returnvalue_4)) (.種族傷害倍率 (Utilities|Struct|BreakST_CharacterInfo_Beast _returnvalue_4)) (.進階攻擊呼叫次數 (Utilities|Struct|BreakST_CharacterInfo_Beast _returnvalue_4))))))
    (:NewEnumerator2
      (bind _returnvalue_5 (Utilities|GetDataTableRow "/Game/_Waraces/Cards/Character_Cards/Datas/DT_Character_Goblin.DT_Character_Goblin" _returnvalue_2)
        (:then
          (return (.攻擊力 (Utilities|Struct|BreakST_CharacterInfo_Goblin _returnvalue_5)) (.攻擊速度 (Utilities|Struct|BreakST_CharacterInfo_Goblin _returnvalue_5)) (.生命值 (Utilities|Struct|BreakST_CharacterInfo_Goblin _returnvalue_5)) (.普攻回魔量 (Utilities|Struct|BreakST_CharacterInfo_Goblin _returnvalue_5)) (.進階攻擊所需魔量 (Utilities|Struct|BreakST_CharacterInfo_Goblin _returnvalue_5)) (.種族傷害倍率 (Utilities|Struct|BreakST_CharacterInfo_Goblin _returnvalue_5)) (.進階攻擊呼叫次數 (Utilities|Struct|BreakST_CharacterInfo_Goblin _returnvalue_5))))))))