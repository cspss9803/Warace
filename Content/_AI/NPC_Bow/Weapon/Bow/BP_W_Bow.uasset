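; Bow weapon Blueprint for the bow NPC that animates its string through a PoseableMesh as the bow is drawn.
; BeginPlay caches the String bone's rest position, and 拉弓 passes the draw flag through a multicast-named event.
; While drawn, Tick snaps the bone to the ArrowLocation socket on the first BP_TakeArrow found in the world, otherwise restoring the rest position.
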(event Custom|拉弓
  (params (是否拉弓 :type Boolean))
  (CallFunction|拉弓Multicast 是否拉弓))

(event Custom|拉弓_Multicast
  (params (是否拉弓 :type Boolean))
  (Variables|Default|Set是否拉弓 是否拉弓))

(event EventBeginPlay
  (bind _returnvalue (Class|PoseableMeshComponent|GetBoneLocationbyName (Variables|Default|GetPoseableMesh) "String" "ComponentSpace"))
  (Variables|Default|Set存取預設位置 _returnvalue))

(event EventTick
  (params (DeltaSeconds :type Float%20%28single-precision%29))
  (bind _poseablemesh (Variables|Default|GetPoseableMesh))
  (if (Variables|Default|Get是否拉弓)
    (bind _returnvalue (Actor|GetActorOfClass "/Game/_AI/_Attack/Projectile/Arrow/BP_TakeArrow.BP_TakeArrow_C"))
    (Class|PoseableMeshComponent|SetBoneLocationbyName _poseablemesh "String" (Transformation|GetSocketLocation (Variables|/Game/_AI/_Attack/Projectile/Arrow/BP_TakeArrow.BP_TakeArrow_C|GetArrow _returnvalue) "ArrowLocation") "WorldSpace")
    (else
      (Class|PoseableMeshComponent|SetBoneLocationbyName _poseablemesh "String" (Variables|Default|Get存取預設位置) "ComponentSpace"))))

(fn ConstructionScript)