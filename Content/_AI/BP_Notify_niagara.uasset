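; Animation notify that spawns attack Niagara effects on NPCs derived from BP_NPC_Base, currently implemented only for the Lava character type.
; It branches on the owner's attack type (攻擊類型), then character type (角色種類), casting to BP_NPC_Lava.
; Normal attacks attach Lava_Dash to the left hand with an offset; advanced attacks attach Lava_ball at the launch socket (發射位置).
; Each effect is tinted with that NPC's color for the attack.
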(fn ReceivedNotify
  (params (MeshComp :type Skeletal%20Mesh%20Component%20Object%20Reference) (Animation :type Anim%20Sequence%20Base%20Object%20Reference) (EventReference :type Anim%20Notify%20Event%20Reference%20Structure%20%28by%20ref%29))
  (bind _returnvalue (Components|GetOwner MeshComp))
  (LocalVariables|SetGetOwner _returnvalue)
  (bind _asbp_npc_base (Utilities|Casting|CastToBP_NPC_Base _returnvalue))
  (switch Utilities|FlowControl|Switch|SwitchonE_AttackData (Variables|/Game/_AI/NPC_Base/BP_NPC_Base.BP_NPC_Base_C|Get攻擊類型 _asbp_npc_base)
    (:NewEnumerator0
      (switch Utilities|FlowControl|Switch|SwitchonE_NPC (Variables|/Game/_AI/NPC_Base/BP_NPC_Base.BP_NPC_Base_C|Get角色種類 _asbp_npc_base)
        (:NewEnumerator4
          (bind _asbp_npc_lava (Utilities|Casting|CastToBP_NPC_Lava (LocalVariables|GetGetOwner)))
          (bind _returnvalue_2 (Niagara|SpawnSystemAttached "/Game/_AI/NPC_Lava/VFX/Lava_Dash.Lava_Dash" (Variables|/Script/Engine.Character|GetMesh _asbp_npc_lava) "LeftHand" "-500.000000,100.000000,0.000000" "0, 0, 0" "KeepRelativeOffset" false))
          (Effects|Components|ParticleSystem|SetColorParameter _returnvalue_2 "Color" (Variables|/Game/_AI/NPC_Base/BP_NPC_Lava.BP_NPC_Lava_C|Get普通攻擊_Color _asbp_npc_lava)))))
    (:NewEnumerator1
      (switch Utilities|FlowControl|Switch|SwitchonE_NPC (Variables|/Game/_AI/NPC_Base/BP_NPC_Base.BP_NPC_Base_C|Get角色種類 _asbp_npc_base)
        (:NewEnumerator4
          (bind _asbp_npc_lava_2 (Utilities|Casting|CastToBP_NPC_Lava (LocalVariables|GetGetOwner)))
          (bind _returnvalue_3 (Niagara|SpawnSystemAttached "/Game/_AI/NPC_Lava/VFX/Lava_ball.Lava_ball" (Variables|/Script/Engine.Character|GetMesh _asbp_npc_lava_2) "發射位置" "0, 0, 0" "0, 0, 0" "KeepRelativeOffset" false))
          (Effects|Components|ParticleSystem|SetColorParameter _returnvalue_3 "Color" (Variables|/Game/_AI/NPC_Base/BP_NPC_Lava.BP_NPC_Lava_C|Get進階攻擊_Color _asbp_npc_lava_2))
          (return false))))))