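; Player controller that handles the player identity check, leaving the game and the timer display in a match.
; 取得身份證 reads the ID from the game instance and passes it through 回傳身份證 to the game mode's 檢查身分證 check, along with the controller itself.
; 離開遊戲 opens Map_Login, and 讓計時介面開始面向玩家 finds BP_Timer and tells it to start turning toward this player.
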(event Custom|離開遊戲
  (Game|OpenLevel(byObjectReference) "/Game/_Waraces/Maps/Map_Login.Map_Login"))

(event Custom|讓計時介面開始面向玩家
  (bind _returnvalue (Actor|GetActorOfClass "/Game/_Waraces/Scene_UIs/MainMap/Timer/BP_Timer.BP_Timer_C"))
  (Default|開始轉向玩家 _returnvalue self))

(event Custom|取得身份證
  (CallFunction|回傳身份證 (Variables|/Game/_Waraces/Blueprints/GamePlay/GI.GI_C|Get身份證 (CallFunction|取得遊戲實例))))

(event Custom|回傳身份證
  (params (身份證 :type Guid%20Structure))
  (Default|檢查身分證 (CallFunction|取得遊戲模式) 身份證 self))

(fn ConstructionScript)