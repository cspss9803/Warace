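; Rock variant of an area-of-effect damage-over-time actor, filed among the beast NPC VFX, that adds rock visuals and sound to the hit.
; Overrides HitActor, noted as one-time damage, to run the parent logic and then the 生成Rock (spawn rock) event.
; That event attaches the P_Rock emitter to the root and plays a rubble sound at the actor's location, intended to show on clients too.
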(event Custom|生成%20Rock
  (Effects|SpawnEmitterAttached "/Game/_Waraces/AI_Charcaters/NPC_Beast/VFXs/Rock/P_Rock.P_Rock" (Variables|Default|GetDefaultSceneRoot) "None")
  (Audio|PlaySoundatLocation "/Game/_Waraces/AI_Charcaters/NPC_Beast/Audio/SW_碎石.SW_碎石" (Transformation|GetActorLocation self) "0, 0, 0" 1.0 1.0 0.0 0 0 0 0))

(event EventBeginPlay
  (|CallParentFunction) ; This node is disabled and will not be called.\nDrag off pins to build functionality.
)

(event Collision|EventActorBeginOverlap
  (params (OtherActor :type Actor%20Object%20Reference))
  (|CallParentFunction OtherActor) ; This node is disabled and will not be called.\nDrag off pins to build functionality.
)

(event EventTick
  (params (DeltaSeconds :type Float%20%28single-precision%29))
  (|CallParentFunction DeltaSeconds) ; This node is disabled and will not be called.\nDrag off pins to build functionality.
)

(event EventHitActor
  (|CallParentFunction)
  (CallFunction|生成Rock))

(fn ConstructionScript
  (|CallParentFunction))