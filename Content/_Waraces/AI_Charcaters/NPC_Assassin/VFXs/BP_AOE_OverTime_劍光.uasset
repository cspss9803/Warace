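; Area-of-effect over-time Blueprint for the NPC Assassin's sword-light (劍光) slash effect.
; A single custom event calls HitActor, then spawns the NS_Slash_CiAb_01 slash effect attached to the root, auto-destroyed when finished.
; The graph holds no timing, targeting or damage logic of its own, and nothing in it triggers the event.
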(event Custom|CustomEvent
  (CallFunction|HitActor)
  (Niagara|SpawnSystemAttached "/Game/_Waraces/AI_Charcaters/NPC_Assassin/VFXs/NiagaraMagicalSlashes/Fx/Slashes/NS_Slash_CiAb_01.NS_Slash_CiAb_01" (Variables|Default|GetDefaultSceneRoot) "None" "0, 0, 0" "0, 0, 0" "KeepRelativeOffset" true))

(event EventBeginPlay
  (|CallParentFunction) ; This node is disabled and will not be called.\nDrag off pins to build functionality.
)

(event Collision|EventActorBeginOverlap
  (params (OtherActor :type Actor%20Object%20Reference))
  (|CallParentFunction OtherActor) ; This node is disabled and will not be called.\nDrag off pins to build functionality.
)

(event EventTick
  (params (DeltaSeconds :type Float%20%28single-precision%29))
  (|CallParentFunction DeltaSeconds) ; This node is disabled and will not be called.\nDrag off pins to build functionality.
)

(fn ConstructionScript
  (|CallParentFunction))